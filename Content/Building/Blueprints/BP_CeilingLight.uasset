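; Ceiling light actor for buildings, pairing a spot light with a lightbulb mesh that can switch on and off.
; On BeginPlay it applies the light color and on/off state to both components.
; Turnon and TurnOff update the spot light intensity and the bulb's emission, which is driven through custom primitive data along with its color.
; The toggle and emission setter events are empty stubs.
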(event EventBeginPlay
  (CallFunction|RefreshLightbulbEmissionColor)
  (CallFunction|RefreshLighbulbEmissionIntensity)
  (CallFunction|RefreshLightIntensity)
  (CallFunction|RefreshLightColor))

(event Collision|EventActorBeginOverlap
  (params (OtherActor :type Actor%20Object%20Reference)))

(event EventTick
  (params (DeltaSeconds :type Float%20%28single-precision%29)))

(event EventTurnon
  (Variables|Default|SetIsOn true)
  (CallFunction|RefreshLighbulbEmissionIntensity)
  (CallFunction|RefreshLightIntensity))

(event EventTurnOff
  (Variables|Default|SetIsOn false)
  (CallFunction|RefreshLighbulbEmissionIntensity)
  (CallFunction|RefreshLightIntensity))

(event EventToggleonOff)

(event EventSetOffEmissionIntensity
  (params (NewOffEmissionIntensity :type Float%20%28double-precision%29)))

(event EventSetonEmissionIntensity
  (params (NewOnEmissionIntensity :type Float%20%28double-precision%29)))

(event EventSetEmissionColor
  (params (NewEmissiveColor :type Linear%20Color%20Structure)))

(fn ConstructionScript)

(fn RefreshLightbulbEmissionColor
  (bind _lightcolor (Variables|Default|GetLightColor))
  (Rendering|Material|SetCustomPrimitiveDataVector4 (Variables|Default|GetLightbulb) 0 (Math|Vector4|MakeVector4 (.r _lightcolor) (.g _lightcolor) (.b _lightcolor) (.a _lightcolor))))

(fn RefreshLighbulbEmissionIntensity
  (bind _lightbulb (Variables|Default|GetLightbulb))
  (if (Variables|Default|GetIsOn)
    (Rendering|Material|SetCustomPrimitiveDataFloat _lightbulb 4 1.0)
    (else
      (Rendering|Material|SetCustomPrimitiveDataFloat _lightbulb 4 0.0))))

(fn RefreshLightIntensity
  (bind _spotlight (Variables|Default|GetSpotLight))
  (if (Variables|Default|GetIsOn)
    (Rendering|Components|Light|SetIntensity _spotlight (Variables|Default|GetOnLightIntensity))
    (else
      (Rendering|Components|Light|SetIntensity _spotlight 0.0))))

(fn RefreshLightColor
  (Rendering|Components|Light|SetLightColor (Variables|Default|GetSpotLight) (Variables|Default|GetLightColor) true))