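; Sliding door actor for buildings that toggles open or closed on interaction and can be locked.
; Interact checks the lock, where key checking is still a TODO, then opens or closes the door based on IsOpen.
; One timeline, played or reversed, slides the door root along local Y and flips IsOpen when finished.
; Separate functions snap the door open or closed instantly, and debug prints report door ID and state.
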(event EventToggleDoorOpen
  (bind _doorid (CallFunction|GetDoorID))
  (bind _islocked (CallFunction|GetIsLocked))
  (Development|PrintString (Utilities|String|Append (Utilities|String|Append (Utilities|String|ToString(Name) _doorid) " isLocked = ") (Utilities|String|ToString(Boolean) _islocked)))
  (if _islocked
    (Development|PrintString "IsLocked TODO:Check if have key")
    (else
      (bind _isopen (CallFunction|GetIsOpen))
      (Development|PrintString (Utilities|String|Append (Utilities|String|Append (Utilities|String|ToString(Name) _doorid) " isOpen =") (Utilities|String|ToString(Boolean) _isopen)))
      (if _isopen
        (CallFunction|CloseDoor)
        (else
          (CallFunction|OpenDoor))))))

(event EventCloseDoor
  (bind _doorlocationy (Timeline|DoorSlideTimeline Reverse)
    (:Update
      (Transformation|SetRelativeLocation (Variables|Default|GetDoorRotationRoot) (Math|Vector|MakeVector 0.0 _doorlocationy 0.0) false false))
    (:Finished
      (CallFunction|SetIsOpen (not (Variables|Default|GetIsOpen))))))

(event EventSetIsLocked
  (params (NewIsLocked :type Boolean))
  (Variables|Default|SetIsLocked NewIsLocked))

(event EventToggleDoorLock
  (Variables|Default|SetIsLocked (not (Variables|Default|GetIsLocked))))

(event EventOpenDoor
  (bind _doorlocationy (Timeline|DoorSlideTimeline Play)
    (:Update
      (Transformation|SetRelativeLocation (Variables|Default|GetDoorRotationRoot) (Math|Vector|MakeVector 0.0 _doorlocationy 0.0) false false))
    (:Finished
      (CallFunction|SetIsOpen (not (Variables|Default|GetIsOpen))))))

(event EventInteract
  (params (PlayerCharacter :type BP%20First%20Person%20Character%20Object%20Reference))
  (CallFunction|ToggleDoorOpen))

(event EventSetIsOpen
  (params (NewIsOpen :type Boolean))
  (Variables|Default|SetIsOpen NewIsOpen))

(event EventSetDoorID
  (params (NewDoorID :type Name :default "None"))
  (Variables|Default|SetDoorID NewDoorID))

(fn ConstructionScript)

(fn SlideDoorOpenInstant
  (Transformation|SetRelativeLocation (Variables|Default|GetDoorRotationRoot) "0.000000,-150.000000,0.000000" false false))

(fn SlideDoorClosedInstant
  (Transformation|SetRelativeLocation (Variables|Default|GetDoorRotationRoot) "0, 0, 0" false false))

(fn GetDoorID
  (return (Variables|Default|GetDoorID)))

(fn GetIsLocked
  (return (Variables|Default|GetIsLocked)))

(fn GetIsOpen
  (return (Variables|Default|GetIsOpen)))