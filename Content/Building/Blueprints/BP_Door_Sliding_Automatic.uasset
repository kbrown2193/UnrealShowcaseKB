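; Automatic sliding door that opens when the player begins overlapping it and closes when the overlap ends.
; A timeline plays or reverses to slide DoorRotationRoot along local Y, flipping IsOpen on finish; overlaps stop any slide in progress before changing direction.
; Interact also toggles the door and respects IsLocked, with the key check still a TODO, while overlap opening ignores the lock.
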(event Custom|StopSliding
  (Variables|Default|SetIsSliding false)
  (bind _doorlocationy (Timeline|DoorSlideTimeline Stop)
    (:Update
      (Transformation|SetRelativeLocation (Variables|Default|GetDoorRotationRoot) (Math|Vector|MakeVector 0.0 _doorlocationy 0.0) false false))
    (:Finished
      (CallFunction|SetIsOpen (not (Variables|Default|GetIsOpen)))
      (Variables|Default|SetIsSliding false))))

(event EventToggleDoorOpen
  (bind _doorid (CallFunction|GetDoorID))
  (bind _islocked (CallFunction|GetIsLocked))
  (Development|PrintString (Utilities|String|Append (Utilities|String|Append (Utilities|String|ToString(Name) _doorid) " isLocked = ") (Utilities|String|ToString(Boolean) _islocked)))
  (if _islocked
    (Development|PrintString "IsLocked TODO:Check if have key")
    (else
      (bind _isopen (CallFunction|GetIsOpen))
      (Development|PrintString (Utilities|String|Append (Utilities|String|Append (Utilities|String|ToString(Name) _doorid) " isOpen =") (Utilities|String|ToString(Boolean) _isopen)))
      (if _isopen
        (CallFunction|CloseDoor)
        (else
          (CallFunction|OpenDoor))))))

(event EventCloseDoor
  (Variables|Default|SetIsSliding true)
  (bind _doorlocationy (Timeline|DoorSlideTimeline Reverse)
    (:Update
      (Transformation|SetRelativeLocation (Variables|Default|GetDoorRotationRoot) (Math|Vector|MakeVector 0.0 _doorlocationy 0.0) false false))
    (:Finished
      (CallFunction|SetIsOpen (not (Variables|Default|GetIsOpen)))
      (Variables|Default|SetIsSliding false))))

(event EventSetIsLocked
  (params (NewIsLocked :type Boolean))
  (Variables|Default|SetIsLocked NewIsLocked))

(event EventToggleDoorLock
  (Variables|Default|SetIsLocked (not (Variables|Default|GetIsLocked))))

(event EventOpenDoor
  (Variables|Default|SetIsSliding true)
  (bind _doorlocationy (Timeline|DoorSlideTimeline Play)
    (:Update
      (Transformation|SetRelativeLocation (Variables|Default|GetDoorRotationRoot) (Math|Vector|MakeVector 0.0 _doorlocationy 0.0) false false))
    (:Finished
      (CallFunction|SetIsOpen (not (Variables|Default|GetIsOpen)))
      (Variables|Default|SetIsSliding false))))

(event EventInteract
  (CallFunction|ToggleDoorOpen))

(event Collision|EventActorBeginOverlap
  (params (OtherActor :type Actor%20Object%20Reference))
  (if (== OtherActor (Game|GetPlayerCharacter 0))
    (if (Variables|Default|GetIsSliding)
      (CallFunction|StopSliding)
      (CallFunction|OpenDoor)
      (else
        (CallFunction|OpenDoor)))))

(event Collision|EventActorEndOverlap
  (params (OtherActor :type Actor%20Object%20Reference))
  (if (== OtherActor (Game|GetPlayerCharacter 0))
    (if (Variables|Default|GetIsSliding)
      (CallFunction|StopSliding)
      (CallFunction|CloseDoor)
      (else
        (CallFunction|CloseDoor)))))

(event EventSetIsOpen
  (params (NewIsOpen :type Boolean))
  (Variables|Default|SetIsOpen NewIsOpen))

(event EventSetDoorID
  (params (NewDoorID :type Name :default "None"))
  (Variables|Default|SetDoorID NewDoorID))

(fn ConstructionScript)

(fn SlideDoorOpenInstant
  (Transformation|SetRelativeLocation (Variables|Default|GetDoorRotationRoot) "0.000000,-150.000000,0.000000" false false))

(fn SlideDoorClosedInstant
  (Transformation|SetRelativeLocation (Variables|Default|GetDoorRotationRoot) "0, 0, 0" false false))

(fn GetDoorID
  (return (Variables|Default|GetDoorID)))

(fn GetIsLocked
  (return (Variables|Default|GetIsLocked)))

(fn GetIsOpen
  (return (Variables|Default|GetIsOpen)))