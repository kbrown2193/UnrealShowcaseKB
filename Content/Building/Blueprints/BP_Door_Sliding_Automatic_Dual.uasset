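; Automatic two-panel sliding door that opens when the player starts overlapping it and closes when the overlap ends.
; One timeline slides both panels along local Y, playing forward or reversed and stopping first if interrupted mid-slide.
; Interact toggles it unless locked, with the key check still TODO; overlap ignores the lock.
; Open and close sounds come from the DT_Doors_Information row matching DoorID.
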(event Custom|StopSliding
  (Variables|Default|SetIsSliding false)
  (bind (_direction _door_l_location_y _door_r_location_y) (Timeline|DoorSlideTimeline Stop)
    (:Update
      (Transformation|SetRelativeLocation (Variables|Default|GetDoor_L_RotationRoot) (Math|Vector|MakeVector 0.0 _door_l_location_y 0.0) false false)
      (Transformation|SetRelativeLocation (Variables|Default|GetDoor_R_RotationRoot) (Math|Vector|MakeVector 0.0 _door_r_location_y 0.0) false false))
    (:Finished
      (CallFunction|SetIsOpen (not (Variables|Default|GetIsOpen)))
      (Variables|Default|SetIsSliding false))))

(event EventToggleDoorOpen
  (bind _doorid (CallFunction|GetDoorID))
  (bind _islocked (CallFunction|GetIsLocked))
  (Development|PrintString (Utilities|String|Append (Utilities|String|Append (Utilities|String|ToString(Name) _doorid) " isLocked = ") (Utilities|String|ToString(Boolean) _islocked)))
  (if _islocked
    (Development|PrintString "IsLocked TODO:Check if have key")
    (else
      (bind _isopen (CallFunction|GetIsOpen))
      (Development|PrintString (Utilities|String|Append (Utilities|String|Append (Utilities|String|ToString(Name) _doorid) " isOpen =") (Utilities|String|ToString(Boolean) _isopen)))
      (if _isopen
        (CallFunction|CloseDoor)
        (else
          (CallFunction|OpenDoor))))))

(event EventCloseDoor
  (Variables|Default|SetIsSliding true)
  (CallFunction|PlaySoundCueViaDoorID (Variables|Default|GetDoorID) false)
  (bind (_direction _door_l_location_y _door_r_location_y) (Timeline|DoorSlideTimeline Reverse)
    (:Update
      (Transformation|SetRelativeLocation (Variables|Default|GetDoor_L_RotationRoot) (Math|Vector|MakeVector 0.0 _door_l_location_y 0.0) false false)
      (Transformation|SetRelativeLocation (Variables|Default|GetDoor_R_RotationRoot) (Math|Vector|MakeVector 0.0 _door_r_location_y 0.0) false false))
    (:Finished
      (CallFunction|SetIsOpen (not (Variables|Default|GetIsOpen)))
      (Variables|Default|SetIsSliding false))))

(event EventSetIsLocked
  (params (NewIsLocked :type Boolean))
  (Variables|Default|SetIsLocked NewIsLocked))

(event EventToggleDoorLock
  (Variables|Default|SetIsLocked (not (Variables|Default|GetIsLocked))))

(event EventOpenDoor
  (Variables|Default|SetIsSliding true)
  (CallFunction|PlaySoundCueViaDoorID (Variables|Default|GetDoorID) true)
  (bind (_direction _door_l_location_y _door_r_location_y) (Timeline|DoorSlideTimeline Play)
    (:Update
      (Transformation|SetRelativeLocation (Variables|Default|GetDoor_L_RotationRoot) (Math|Vector|MakeVector 0.0 _door_l_location_y 0.0) false false)
      (Transformation|SetRelativeLocation (Variables|Default|GetDoor_R_RotationRoot) (Math|Vector|MakeVector 0.0 _door_r_location_y 0.0) false false))
    (:Finished
      (CallFunction|SetIsOpen (not (Variables|Default|GetIsOpen)))
      (Variables|Default|SetIsSliding false))))

(event EventInteract
  (params (PlayerCharacter :type BP%20First%20Person%20Character%20Object%20Reference))
  (CallFunction|ToggleDoorOpen))

(event Collision|EventActorBeginOverlap
  (params (OtherActor :type Actor%20Object%20Reference))
  (if (== OtherActor (Game|GetPlayerCharacter 0))
    (if (Variables|Default|GetIsSliding)
      (CallFunction|StopSliding)
      (CallFunction|OpenDoor)
      (else
        (CallFunction|OpenDoor)))))

(event Collision|EventActorEndOverlap
  (params (OtherActor :type Actor%20Object%20Reference))
  (if (== OtherActor (Game|GetPlayerCharacter 0))
    (if (Variables|Default|GetIsSliding)
      (CallFunction|StopSliding)
      (CallFunction|CloseDoor)
      (else
        (CallFunction|CloseDoor)))))

(event EventSetIsOpen
  (params (NewIsOpen :type Boolean))
  (Variables|Default|SetIsOpen NewIsOpen))

(event EventSetDoorID
  (params (NewDoorID :type Name :default "None"))
  (Variables|Default|SetDoorID NewDoorID))

(fn ConstructionScript)

(fn SlideDoorOpenInstant
  (Transformation|SetRelativeLocation (Variables|Default|GetDoor_L_RotationRoot) "0.000000,-150.000000,0.000000" false false))

(fn SlideDoorClosedInstant
  (Transformation|SetRelativeLocation (Variables|Default|GetDoor_L_RotationRoot) "0, 0, 0" false false))

(fn PlaySoundCueViaDoorID
  (params (DoorID :type Name) (IsOpenSound :type Boolean))
  (bind _defaultsceneroot (Variables|Default|GetDefaultSceneRoot))
  (bind _returnvalue (Transformation|GetWorldLocation _defaultsceneroot))
  (bind _returnvalue_2 (Utilities|GetDataTableRow "/Game/Building/Data/DT_Doors_Information.DT_Doors_Information" DoorID)
    (:then
      (if IsOpenSound
        (Audio|PlaySoundatLocation (.DoorOpenSoundCue (Utilities|Struct|BreakS_Door_Information _returnvalue_2)) _returnvalue "0, 0, 0" 1.0 1.0 0.0 0 0 0 0)
        (else
          (Audio|PlaySoundatLocation (.DoorCloseSoundCue (Utilities|Struct|BreakS_Door_Information _returnvalue_2)) _returnvalue "0, 0, 0" 1.0 1.0 0.0 0 0 0 0))))))

(fn GetDoorID
  (return (Variables|Default|GetDoorID)))

(fn GetIsLocked
  (return (Variables|Default|GetIsLocked)))

(fn GetIsOpen
  (return (Variables|Default|GetIsOpen)))