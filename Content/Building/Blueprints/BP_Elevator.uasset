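; Elevator actor with two sliding doors that toggle open and closed, a lock state, a door ID and a floor text display.
; ToggleDoorOpen checks the lock, then plays or reverses a timeline that slides both door roots and flips IsOpen when finished.
; AttemptToGoToFloor only prints whether the door is closed, with no movement yet, and the key check is a TODO.
; Interact is empty and the old overlap-based automatic opening is disconnected.
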(event Custom|StopSliding
  (Variables|Default|SetIsSliding false)
  (bind (_direction _door_l_location_y _door_r_location_y) (Timeline|DoorSlideTimeline Stop)
    (:Update
      (Transformation|SetRelativeLocation (Variables|Default|GetDoor_L_RotationRoot) (Math|Vector|MakeVector 0.0 _door_l_location_y 0.0) false false)
      (Transformation|SetRelativeLocation (Variables|Default|GetDoor_R_RotationRoot) (Math|Vector|MakeVector 0.0 _door_r_location_y 0.0) false false))
    (:Finished
      (CallFunction|SetIsOpen (not (Variables|Default|GetIsOpen)))
      (Variables|Default|SetIsSliding false))))

(event Custom|AttemptToGoToFloor
  (params (Floor :type Integer))
  (if (Variables|Default|GetIsOpen)
    (Development|PrintString "Elevator Door is open, need to close")
    (else
      (Development|PrintString (Utilities|String|Append "Elevator Door is closed, begin going to floor" (Utilities|String|ToString(Integer) Floor))))))

(event EventToggleDoorOpen
  (bind _doorid (CallFunction|GetDoorID))
  (bind _islocked (CallFunction|GetIsLocked))
  (Development|PrintString (Utilities|String|Append (Utilities|String|Append (Utilities|String|ToString(Name) _doorid) " isLocked = ") (Utilities|String|ToString(Boolean) _islocked)))
  (if _islocked
    (Development|PrintString "IsLocked TODO:Check if have key")
    (else
      (bind _isopen (CallFunction|GetIsOpen))
      (Development|PrintString (Utilities|String|Append (Utilities|String|Append (Utilities|String|ToString(Name) _doorid) " isOpen =") (Utilities|String|ToString(Boolean) _isopen)))
      (if _isopen
        (CallFunction|CloseDoor)
        (else
          (CallFunction|OpenDoor))))))

(event EventCloseDoor
  (Variables|Default|SetIsSliding true)
  (bind (_direction _door_l_location_y _door_r_location_y) (Timeline|DoorSlideTimeline Reverse)
    (:Update
      (Transformation|SetRelativeLocation (Variables|Default|GetDoor_L_RotationRoot) (Math|Vector|MakeVector 0.0 _door_l_location_y 0.0) false false)
      (Transformation|SetRelativeLocation (Variables|Default|GetDoor_R_RotationRoot) (Math|Vector|MakeVector 0.0 _door_r_location_y 0.0) false false))
    (:Finished
      (CallFunction|SetIsOpen (not (Variables|Default|GetIsOpen)))
      (Variables|Default|SetIsSliding false))))

(event EventSetIsLocked
  (params (NewIsLocked :type Boolean))
  (Variables|Default|SetIsLocked NewIsLocked))

(event EventToggleDoorLock
  (Variables|Default|SetIsLocked (not (Variables|Default|GetIsLocked))))

(event EventOpenDoor
  (Variables|Default|SetIsSliding true)
  (bind (_direction _door_l_location_y _door_r_location_y) (Timeline|DoorSlideTimeline Play)
    (:Update
      (Transformation|SetRelativeLocation (Variables|Default|GetDoor_L_RotationRoot) (Math|Vector|MakeVector 0.0 _door_l_location_y 0.0) false false)
      (Transformation|SetRelativeLocation (Variables|Default|GetDoor_R_RotationRoot) (Math|Vector|MakeVector 0.0 _door_r_location_y 0.0) false false))
    (:Finished
      (CallFunction|SetIsOpen (not (Variables|Default|GetIsOpen)))
      (Variables|Default|SetIsSliding false))))

(event EventInteract
  (params (PlayerCharacter :type BP%20First%20Person%20Character%20Object%20Reference))
  ;[1 1 1] OLD Trigger Based Automatic Opening
)

(event Collision|EventActorBeginOverlap
  (params (OtherActor :type Actor%20Object%20Reference))
  ;[1 1 1] OLD Trigger Based Automatic Opening
)

(event Collision|EventActorEndOverlap
  (params (OtherActor :type Actor%20Object%20Reference))
  ;[1 1 1] OLD Trigger Based Automatic Opening
)

(event EventSetIsOpen
  (params (NewIsOpen :type Boolean))
  (Variables|Default|SetIsOpen NewIsOpen))

(event EventSetDoorID
  (params (NewDoorID :type Name :default "None"))
  (Variables|Default|SetDoorID NewDoorID))

(fn ConstructionScript)

(fn SlideDoorOpenInstant
  (Transformation|SetRelativeLocation (Variables|Default|GetDoor_L_RotationRoot) "0.000000,-150.000000,0.000000" false false))

(fn SlideDoorClosedInstant
  (Transformation|SetRelativeLocation (Variables|Default|GetDoor_L_RotationRoot) "0, 0, 0" false false))

(fn SetFloorText
  (params (Text%20Value :type Text))
  (Rendering|Components|TextRender|SetText (Variables|Default|GetFloorTextRender) Text%20Value))

(fn GetDoorID
  (return (Variables|Default|GetDoorID)))

(fn GetIsLocked
  (return (Variables|Default|GetIsLocked)))

(fn GetIsOpen
  (return (Variables|Default|GetIsOpen)))