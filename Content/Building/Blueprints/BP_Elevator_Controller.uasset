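; BP_Elevator_Controller receives button requests for a building elevator and drives the car and floor doors.
; ElevatorButtonRequest switches on the button type and prints a debug message for each press.
; Only up or down call buttons act, opening that floor's door and the elevator door when the car is already at that floor.
; Door, floor and alarm buttons only log, and no travel logic exists here.
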(event EventBeginPlay)

(event Collision|EventActorBeginOverlap
  (params (OtherActor :type Actor%20Object%20Reference)))

(event EventTick
  (params (DeltaSeconds :type Float%20%28single-precision%29)))

(fn ConstructionScript)

(fn ElevatorButtonRequest
  (params (Elevator%20Control%20Button%20Type :type E_ElevatorControlButton%20Enum :default "NewEnumerator0") (Button%20Value :type Integer))
  (bind _returnvalue (Utilities|String|ToString(Integer) Button%20Value))
  (bind _currentfloor (Variables|Default|GetCurrentFloor))
  (bind _elevatorfloordoors (Variables|Default|GetElevatorFloorDoors))
  (bind _elevator (Variables|Default|GetElevator))
  (bind _output (Utilities|Array|Get(acopy) _elevatorfloordoors Button%20Value))
  (bind _returnvalue_2 (== Button%20Value _currentfloor))
  (switch Utilities|FlowControl|Switch|SwitchonE_ElevatorControlButton Elevator%20Control%20Button%20Type
    (:NewEnumerator0
      (Development|PrintString (Utilities|String|Append "Elevator Door Open  Button " _returnvalue)))
    (:NewEnumerator1
      (Development|PrintString (Utilities|String|Append "Elevator Door Close  Button " _returnvalue)))
    (:NewEnumerator2
      (Development|PrintString (Utilities|String|Append "Elevator Floor  Button " _returnvalue)))
    (:NewEnumerator3
      (Development|PrintString (Utilities|String|Append "Elevator Request Down Button Pesssed at floor " _returnvalue))
      (if _returnvalue_2
        (Default|OpenDoor _output)
        (Default|OpenDoor _elevator)))
    (:NewEnumerator4
      (Development|PrintString (Utilities|String|Append "Elevator Request Up Button Pesssed at floor " _returnvalue))
      (if _returnvalue_2
        (Default|OpenDoor _output)
        (Default|OpenDoor _elevator)))
    (:NewEnumerator5
      (Development|PrintString "Elevator Alarm Button PRessted"))))