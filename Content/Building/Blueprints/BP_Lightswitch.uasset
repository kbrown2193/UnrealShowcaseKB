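; BP_Lightswitch is an interactable light switch that turns a building's lights on and off through an EmissiveController reference.
; Interact toggles IsOn and plays or reverses a timeline that rolls the switch's root component.
; When the timeline finishes in either direction, it calls TurnAllLightsOn or TurnAllLightsOff on the controller, so lights change only after the flip animation completes.
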(event Custom|ToggleLightSwitch
  (if (Variables|Default|GetIsOn)
    (CallFunction|FlipOff)
    (else
      (CallFunction|Flipon))))

(event Custom|FlipOn
  (bind _emissivecontroller (Variables|Default|GetEmissiveController))
  (Variables|Default|SetIsOn true)
  (bind _lightswitchrotatortrack (Timeline|LightswitchTimeline Play)
    (:Update
      (Transformation|SetRelativeRotation (Variables|Default|GetLightswitch_Root) (Math|Rotator|MakeRotator _lightswitchrotatortrack 0.0 0.0) false false))
    (:Finished
      (if (Variables|Default|GetIsOn)
        (Default|TurnAllLightson _emissivecontroller)
        (else
          (Default|TurnAllLightsOff _emissivecontroller))))))

(event Custom|FlipOff
  (bind _emissivecontroller (Variables|Default|GetEmissiveController))
  (Variables|Default|SetIsOn false)
  (bind _lightswitchrotatortrack (Timeline|LightswitchTimeline Reverse)
    (:Update
      (Transformation|SetRelativeRotation (Variables|Default|GetLightswitch_Root) (Math|Rotator|MakeRotator _lightswitchrotatortrack 0.0 0.0) false false))
    (:Finished
      (if (Variables|Default|GetIsOn)
        (Default|TurnAllLightson _emissivecontroller)
        (else
          (Default|TurnAllLightsOff _emissivecontroller))))))

(event EventInteract
  (CallFunction|ToggleLightSwitch))

(event EventBeginPlay)

(fn ConstructionScript)