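; Analog wall clock decoration that rotates hour, minute and second hand components to show a stored time.
; While IsTicking, Tick advances Seconds by DeltaSeconds scaled by TimeMultiplier, cascading rollovers into Minutes and 12-hour Hours.
; The minute rollover tests against 0 instead of 60, so Hours advances early.
; BeginPlay poses only the hour hand, and SetTime stores values without moving the hands.
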(event EventBeginPlay
  (CallFunction|SetHourHandPosition (Variables|Default|GetHours) (Variables|Default|GetMinutes) (Variables|Default|GetSeconds)))

(event EventTick
  (params (DeltaSeconds :type Float%20%28single-precision%29))
  (if (Variables|Default|GetIsTicking)
    (Variables|Default|SetSeconds (+ (Variables|Default|GetSeconds) (* (Variables|Default|GetTimeMultiplier) DeltaSeconds)))
    (if (< (+ (Variables|Default|GetSeconds) (* (Variables|Default|GetTimeMultiplier) DeltaSeconds)) 6e+01)
      (CallFunction|SetSecondHandPosition (Variables|Default|GetSeconds))
      (elif (< (* DeltaSeconds (Variables|Default|GetTimeMultiplier)) 6e+01)
        (Variables|Default|SetSeconds (- (Variables|Default|GetSeconds) 6e+01))
        (Math|Float|IncrementFloat (Variables|Default|GetMinutes)
          (:%20%20
            (if (< (Variables|Default|GetMinutes) 0.0)
              (CallFunction|SetMinuteHandPosition (Variables|Default|GetMinutes) (Variables|Default|GetSeconds))
              (CallFunction|SetSecondHandPosition (Variables|Default|GetSeconds))
              (else
                (Variables|Default|SetMinutes (- (Variables|Default|GetMinutes) 6e+01))
                (Math|Float|IncrementFloat (Variables|Default|GetHours)
                  (:%20%20
                    (if (< (Variables|Default|GetHours) 12.0)
                      (CallFunction|SetHandsPositions (Variables|Default|GetHours) (Variables|Default|GetMinutes) (Variables|Default|GetSeconds))
                      (else
                        (Variables|Default|SetHours (- (Variables|Default|GetHours) 12.0))
                        (CallFunction|SetHandsPositions (Variables|Default|GetHours) (Variables|Default|GetMinutes) (Variables|Default|GetSeconds))))))))))
        (else
          (Development|PrintString "Delta* TimeMultiplier cannot be greater than 60"))))))

(fn ConstructionScript)

(fn SetHourHandPosition
  (params (Hour :type Float%20%28double-precision%29) (Minute :type Float%20%28double-precision%29) (Second :type Float%20%28double-precision%29))
  (Transformation|SetRelativeRotation (Variables|Default|GetHand_Hours) (Math|Rotator|MakeRotator 0.0 (* (+ (+ (/ Hour 12.0) (/ Minute 7.2e+02)) (/ Second 4.32e+04)) -3.6e+02) 0.0) false false))

(fn SetHandsPositions
  (params (Hours :type Float%20%28double-precision%29) (Minutes :type Float%20%28double-precision%29) (Seconds :type Float%20%28double-precision%29))
  (CallFunction|SetHourHandPosition Hours Minutes Seconds)
  (CallFunction|SetMinuteHandPosition Minutes Seconds)
  (CallFunction|SetSecondHandPosition Seconds))

(fn SetMinuteHandPosition
  (params (Minutes :type Float%20%28double-precision%29) (Seconds :type Float%20%28double-precision%29))
  (Transformation|SetRelativeRotation (Variables|Default|GetHand_Minutes) (Math|Rotator|MakeRotator 0.0 (* (+ (/ Minutes 6e+01) (/ Seconds 3.6e+03)) -3.6e+02) 0.0) false false))

(fn SetSecondHandPosition
  (params (Seconds :type Float%20%28double-precision%29))
  (Transformation|SetRelativeRotation (Variables|Default|GetHand_Seconds) (Math|Rotator|MakeRotator 0.0 (* (/ Seconds 6e+01) -3.6e+02) 0.0) false false))

(fn SetTime
  (params (NewHours :type Float%20%28double-precision%29) (NewMinutes :type Float%20%28double-precision%29) (NewSeconds :type Float%20%28double-precision%29))
  (Variables|Default|SetHours NewHours)
  (Variables|Default|SetMinutes NewMinutes)
  (Variables|Default|SetSeconds NewSeconds))

(fn SetIsTicking
  (params (NewIsTicking :type Boolean))
  (Variables|Default|SetIsTicking NewIsTicking))