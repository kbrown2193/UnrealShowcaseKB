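; BP_StreetLightController switches street lights on and off according to the in-game hour.
; On BeginPlay it can optionally gather every BP_StreetLight in the level into its StreetLights array.
; While ticking is enabled, it polls TimeManager, turning lights off between the off and on hours and on from the on hour.
; An IsOn flag limits the switching calls to state changes, which also print debug messages.
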(event EventBeginPlay
  (bind _streetlights (Variables|Default|GetStreetLights))
  (if (Variables|Default|GetIsFindingAllOnStart)
    (bind _outactors (Actor|GetAllActorsOfClass "/Game/Decoration/Blueprints/BP_StreetLight.BP_StreetLight_C"))
    (Utilities|Array|Resize _streetlights (Utilities|Array|Length _outactors))
    (for (_array_element _array_index) _outactors
      (Utilities|Array|SetArrayElem _streetlights _array_index _array_element))))

(event Collision|EventActorBeginOverlap
  (params (OtherActor :type Actor%20Object%20Reference)))

(event EventTick
  (params (DeltaSeconds :type Float%20%28single-precision%29))
  (bind _timemanager (Variables|Default|GetTimeManager))
  (if (Variables|Default|GetIsTicking)
    (if (Variables|Default|GetIsOn)
      (bind _hours (Default|GetTime _timemanager))
      (if (and (>= _hours (Variables|Default|GetTurnOffTimeHour)) (< _hours (Variables|Default|GetTurnOnTimeHour)))
        (CallFunction|TurnAllStreetLightsOff)
        (Development|PrintString "Turning All Street Lights Off" true true "(R=0.000000,G=0.660000,B=1.000000,A=1.000000)" 1e+01))
      (else
        (bind _hours_2 (Default|GetTime _timemanager))
        (if (>= _hours_2 (Variables|Default|GetTurnOnTimeHour))
          (CallFunction|TurnAllStreetLightson)
          (Development|PrintString "Turning All Street Lights On"))))))

(fn ConstructionScript)

(fn TurnAllStreetLightson
  (for _array_element (Variables|Default|GetStreetLights)
    (Default|TurnonStreetLight _array_element))
  (Variables|Default|SetIsOn true))

(fn TurnAllStreetLightsOff
  (for _array_element (Variables|Default|GetStreetLights)
    (Default|TurnOffStreetLight _array_element))
  (Variables|Default|SetIsOn false))