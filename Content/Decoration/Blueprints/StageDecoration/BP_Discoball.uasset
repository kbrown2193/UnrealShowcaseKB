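; BP_Discoball is a stage decoration that spins a disco ball mesh continuously around its yaw axis.
; On BeginPlay it sets the timeline play rate from a start variable, then plays a looping rotation timeline that restarts itself when finished.
; Each timeline update writes the curve value to the Discoball's relative rotation, and a custom event lets the play rate change.
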(event Custom|RotateLoop
  (bind _rotatez (Timeline|DiscoballRotateLoop PlayFromStart)
    (:Update
      (Transformation|SetRelativeRotation (Variables|Default|GetDiscoball) (Math|Rotator|MakeRotator 0.0 0.0 _rotatez) false false))
    (:Finished
      (CallFunction|RotateLoop))))

(event Custom|Set12sRoationPlayRate
  (params (NewParam :type Float%20%28double-precision%29))
  (Components|Timeline|SetPlayRate (Variables|Default|GetDiscoballRotateLoop) NewParam))

(event EventBeginPlay
  (CallFunction|Set12sRoationPlayRate (Variables|Default|GetStart12sLoopPlayRate))
  (CallFunction|RotateLoop))

(fn ConstructionScript)