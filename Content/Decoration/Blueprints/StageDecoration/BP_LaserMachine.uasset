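; Stage decoration laser machine that, when switched on, shows a timed beam each time FireBeam is called.
; FireBeam line-traces forward from the rotatable CenterRoot and stretches and centers LaserCylinder to the hit distance, with debug trace and hit printouts.
; FadeOutBeam simply hides the cylinder after BeamHoldTime.
; Nothing here triggers firing: BeginPlay and BeamPre are empty, and the pre-fire sequence is disconnected.
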(event Custom|RotateCenter
  (params (TargetRotation :type Rotator))
  (Transformation|SetRelativeRotation (Variables|Default|GetCenterRoot) TargetRotation false false))

(event Custom|FireBeam
  (bind _laser_cylinder (Variables|Default|GetLaser_Cylinder))
  (bind _centerroot (Variables|Default|GetCenterRoot))
  (bind _beamwidth (Variables|Default|GetBeamWidth))
  (bind _returnvalue (Transformation|GetWorldLocation _centerroot))
  (if (Variables|Default|GetIsOn)
    (bind _outhit (Collision|LineTraceByChannel _returnvalue (+ _returnvalue (* (Math|Vector|GetForwardVector (Transformation|GetWorldRotation _centerroot)) (Variables|Default|GetBeamDistance))) "TraceTypeQuery4" false 0 "ForDuration"))
    (Transformation|SetRelativeScale3D _laser_cylinder (Math|Vector|MakeVector _beamwidth _beamwidth (/ (.Distance (Collision|BreakHitResult _outhit)) 1e+02)))
    (Transformation|SetRelativeLocation _laser_cylinder (Math|Vector|MakeVector (/ (.Distance (Collision|BreakHitResult _outhit)) 2.0) 0.0 0.0) false false)
    (Development|PrintString (Utilities|String|BuildString(Vector) (Utilities|String|BuildString(Vector) "" "Laser Hit at " (.ImpactPoint (Collision|BreakHitResult _outhit))) " with normal " (.Normal (Collision|BreakHitResult _outhit))) true true "(R=0.020588,G=0.218750,B=0.000000,A=1.000000)")
    (Development|PrintString (Class|KismetStringLibrary|BuildStringDouble "" "with Distance of " (.Distance (Collision|BreakHitResult _outhit))) true true "(R=0.020588,G=0.218750,B=0.000000,A=1.000000)")
    (Rendering|SetVisibility (Variables|Default|GetLaser_Cylinder) true false)
    (CallFunction|FadeOutBeam)))

(event Custom|BeamPre)

(event Custom|TurnOn
  (Variables|Default|SetIsOn true))

(event Custom|TurnOff
  (Variables|Default|SetIsOn false))

(event Custom|ToggleOnOff
  (if (Variables|Default|GetIsOn)
    (Variables|Default|SetIsOn false)
    (else
      (Variables|Default|SetIsOn true))))

(event Custom|FadeOutBeam
  (Utilities|FlowControl|Delay (Variables|Default|GetBeamHoldTime))
  (Rendering|SetVisibility (Variables|Default|GetLaser_Cylinder) false false))

(event EventBeginPlay)

(fn ConstructionScript)