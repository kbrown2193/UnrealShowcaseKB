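; BP_LaserMachine_Controller is a stage decoration Blueprint that drives a group of laser machines together.
; On BeginPlay, if IsOn is set, it primes every machine with BeamPre and then immediately fires all beams.
; A separate event rotates each machine's center, pairing the LaserMachines and LaserMachineRotations arrays by index.
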(event Custom|RotateAllLaserMachines
  (for (_array_element _array_index) (Variables|Default|GetLaserMachines)
    (Default|RotateCenter _array_element (Utilities|Array|Get(acopy) (Variables|Default|GetLaserMachineRotations) _array_index))))

(event Custom|BeamsPre
  (for _array_element (Variables|Default|GetLaserMachines)
    (Default|BeamPre _array_element)))

(event Custom|FireBeams
  (for _array_element (Variables|Default|GetLaserMachines)
    (Default|FireBeam _array_element)))

(event EventBeginPlay
  (if (Variables|Default|GetIsOn)
    (CallFunction|BeamsPre)
    (CallFunction|FireBeams)))

(fn ConstructionScript)