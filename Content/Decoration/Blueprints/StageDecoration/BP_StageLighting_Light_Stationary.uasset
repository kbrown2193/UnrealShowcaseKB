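; Stationary stage light decoration that pairs a spotlight with an emissive sphere mesh.
; On BeginPlay it re-applies the spotlight's own color and feeds the root's world rotation back as its relative rotation, through custom events.
; The sphere's glow is written to custom primitive data, taking green, blue and alpha from the light color but red from a separate EmissionMeshR variable.
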(event Custom|SetSpotlightColor
  (params (NewParam :type Color%20Structure))
  (Rendering|Components|Light|SetLightColor (Variables|Default|GetSpotLight) (Math|Conversions|ToLinearColor(Color) NewParam) true))

(event Custom|SetRootRotation
  (params (NewParam :type Rotator))
  (Transformation|SetRelativeRotation (Variables|Default|GetDefaultSceneRoot) NewParam false false))

(event Custom|SetMeshEmissionColor
  (params (EmissiveR :type Float%20%28double-precision%29) (EmissiveG :type Float%20%28double-precision%29) (EmissiveB :type Float%20%28double-precision%29) (EmissiveA :type Float%20%28double-precision%29))
  (Rendering|Material|SetCustomPrimitiveDataVector4 (Variables|Default|GetSphere) 0 (Math|Vector4|MakeVector4 EmissiveR EmissiveG EmissiveB EmissiveA)))

(event EventBeginPlay
  (bind _spotlight (Variables|Default|GetSpotLight))
  (bind _lightcolor (Variables|/Script/Engine.LightComponentBase|GetLightColor _spotlight))
  (bind (_b _g _r _a) (Math|Color|BreakColor _lightcolor))
  (CallFunction|SetSpotlightColor _lightcolor)
  (CallFunction|SetRootRotation (Transformation|GetWorldRotation (Variables|Default|GetDefaultSceneRoot)))
  (CallFunction|SetMeshEmissionColor (Variables|Default|GetEmissionMeshR) (Math|Conversions|ToFloat(Byte) _g) (Math|Conversions|ToFloat(Byte) _b) (Math|Conversions|ToFloat(Byte) _a)))

(fn ConstructionScript)