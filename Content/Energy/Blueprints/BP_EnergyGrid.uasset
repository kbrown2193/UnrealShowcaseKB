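; BP_EnergyGrid is an actor that keeps a registry of the energy components that make up an energy grid.
; On BeginPlay it pulls the EnergyComponent from each actor in EnergyObjectActors into its component list, then prints each one's type, consumption, generation and storage.
; Add and remove functions change the list at runtime and print the result, but no energy balancing is computed here.
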(event EventBeginPlay
  (CallFunction|InitializeEnergyComponents)
  (CallFunction|DebugPrintEnergyComponents))

(event Collision|EventActorBeginOverlap
  (params (OtherActor :type Actor%20Object%20Reference)))

(event EventTick
  (params (DeltaSeconds :type Float%20%28single-precision%29)))

(fn ConstructionScript)

(fn AddEnergyObjecttoGrid
  (params (EnergyObjectToAdd :type Energy%20Component%20Object%20Reference))
  (Utilities|Array|Add (Variables|Default|GetEnergyObjectComponents) EnergyObjectToAdd)
  (Development|PrintString "Added to Energy Grid"))

(fn RemoveEnergyObjectfromGrid
  (params (EnergyObjectToRemove :type Energy%20Component%20Object%20Reference))
  (bind _returnvalue (Utilities|Array|RemoveItem (Variables|Default|GetEnergyObjectComponents) EnergyObjectToRemove))
  (if _returnvalue
    (Development|PrintString "Was Removed from energy grid")
    (else
      (Development|PrintString "USnable to remove as was not found in energy grid" true true "(R=1.000000,G=0.974000,B=0.000000,A=1.000000)"))))

(fn InitializeEnergyComponents
  (for _array_element (Variables|Default|GetEnergyObjectActors)
    (Utilities|Array|Add (Variables|Default|GetEnergyObjectComponents) (Actor|GetComponentbyClass _array_element "/Game/Energy/Blueprints/EnergyComponent.EnergyComponent_C"))))

(fn DebugPrintEnergyComponents
  (for (_array_element _array_index) (Variables|Default|GetEnergyObjectComponents)
    (Development|PrintString (Utilities|String|Append "Energy Component[" (Utilities|String|ToString(Integer) _array_index) "] = " (Utilities|GetObjectName _array_element) ", Type = " (Utilities|String|EnumtoString (Variables|/Game/Energy/Blueprints/EnergyComponent.EnergyComponent_C|GetEnergyObjectType _array_element)) ", Consumption = " (Utilities|String|ToString(Float) (Variables|/Game/Energy/Blueprints/EnergyComponent.EnergyComponent_C|GetConsumptionRate _array_element)) ", Generation = " (Utilities|String|ToString(Float) (Variables|/Game/Energy/Blueprints/EnergyComponent.EnergyComponent_C|GetGenerationRate _array_element)) ", Storage = " (Utilities|String|ToString(Float) (Variables|/Game/Energy/Blueprints/EnergyComponent.EnergyComponent_C|GetStorage _array_element))) true true "(R=0.000000,G=0.660000,B=1.000000,A=1.000000)" 6.0)))