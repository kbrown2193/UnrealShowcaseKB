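; BP_WindTurbine is a wind turbine actor that spins its rotation root while IsActive is set.
; A timeline drives the root's relative roll, starting on BeginPlay and restarting from RotateTurbine each time it finishes, as long as the turbine remains active.
; RotationSpeed sets the timeline's play rate, and SetWindTurbineSpeed updates both at runtime.
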(event Custom|RotateTurbine
  (if (Variables|Default|GetIsActive)
    (bind _rotx (Timeline|WindTurbineRotationTimeline PlayFromStart)
      (:Update
        (Transformation|SetRelativeRotation (Variables|Default|GetWindTurbineRotationRoot) (Math|Rotator|MakeRotator _rotx 0.0 0.0) false false))
      (:Finished
        (CallFunction|RotateTurbine)))))

(event EventBeginPlay
  (Components|Timeline|SetPlayRate (Variables|Default|GetWindTurbineRotationTimeline) (Variables|Default|GetRotationSpeed))
  (if (Variables|Default|GetIsActive)
    (bind _rotx (Timeline|WindTurbineRotationTimeline Play)
      (:Update
        (Transformation|SetRelativeRotation (Variables|Default|GetWindTurbineRotationRoot) (Math|Rotator|MakeRotator _rotx 0.0 0.0) false false))
      (:Finished
        (CallFunction|RotateTurbine)))))

(fn ConstructionScript)

(fn SetWindTurbineSpeed
  (params (RotateSpeed :type Float%20%28double-precision%29))
  (bind _output_get (Variables|Default|SetRotationSpeed RotateSpeed))
  (Components|Timeline|SetPlayRate (Variables|Default|GetWindTurbineRotationTimeline) _output_get))