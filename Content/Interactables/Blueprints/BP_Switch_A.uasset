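; BP_Switch_A is an interactable switch that flips between on and off.
; Each Interact event toggles IsOn and snaps the RotationPlane component between two mirrored tilt angles, with no interpolation.
; A DoOnce gate wraps the toggle but resets straight after each flip.
; The switch triggers nothing else in this graph, and a skeletal mesh animation call is left disconnected.
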(event EventInteract
  (Utilities|FlowControl|DoOnce false :!label _label
    (:Completed
      (if (Variables|Default|GetIsOn)
        (Variables|Default|SetIsOn false)
        (Transformation|SetRelativeRotation (Variables|Default|GetRotationPlane) "0.000000,0.000000,45.000000" false false)
        (goto _label Reset)
        (else
          (Variables|Default|SetIsOn true)
          (Transformation|SetRelativeRotation (Variables|Default|GetRotationPlane) "0.000000,0.000000,-45.000000" false false)
          (goto _label Reset))))))

(fn ConstructionScript)