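; Inventory component that stores items in a fixed-size array of slots, with debug keys to print or clear it.
; Adding fills matching stacks one unit at a time up to the DT_ItemData stack size, then uses empty slots, returning any remainder.
; A server event swaps slots between inventories when item IDs differ, then fires MC_Update on both to broadcast OnInventoryUpdated.
; RemoveFromInventory is an empty stub.
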(event Custom|MC_Update
  (Default|CallOnInventoryUpdated))

(event Custom|SERVER_TransferSlots
  (params (SourceIndex :type Integer) (SourceInventorySystem :type BPC%20Inventory%20Object%20Reference) (DestinationIndex :type Integer))
  (CallFunction|TransferSlots SourceIndex SourceInventorySystem DestinationIndex))

(event EventBeginPlay
  (Utilities|Array|Resize (Variables|Default|GetInventoryContent) (Variables|Default|GetInventorySize)))

(event Input|KeyboardEvents|1
  (params (Key :type Key%20Structure :default "None"))
  ;[1 1 1] Debug
  (:Pressed
    (CallFunction|DebugPrintContent)))

(event Input|KeyboardEvents|2
  (params (Key :type Key%20Structure :default "None"))
  ;[1 1 1] Debug
  (:Pressed
    (CallFunction|ClearInventory)))

(fn AddtoInventory
  (params (ItemID :type Name) (Quantity :type Integer))
  (LocalVariables|SetLocalQuantityRemaining Quantity)
  (while (and (> (LocalVariables|GetLocalQuantityRemaining) 0) (not (LocalVariables|GetLocalHasFailed)))
    (bind (_inventoryindex _isslotfound) (CallFunction|FindSlot ItemID))
    (if _isslotfound
      (CallFunction|AddtoStack _inventoryindex 1)
      (Math|Integer|DecrementInt (LocalVariables|GetLocalQuantityRemaining))
      (elif (.HasEmptySlot (CallFunction|AnyEmptySlotsAvailable))
        (bind _wassuccessful (CallFunction|CreateNewStack ItemID 1))
        (if _wassuccessful
          (Math|Integer|DecrementInt (LocalVariables|GetLocalQuantityRemaining))
          (else
            (LocalVariables|SetLocalHasFailed true)))
        (else
          (LocalVariables|SetLocalHasFailed true)))))
  (return (not (LocalVariables|GetLocalHasFailed)) (LocalVariables|GetLocalQuantityRemaining)))

(fn RemovefromInventory)

(fn FindSlot
  (params (ItemID :type Name))
  (for (_array_element _array_index) (Variables|Default|GetInventoryContent)
    (if (== (.ItemID (Utilities|Struct|BreakBPS_ItemSlot _array_element)) ItemID)
      (if (< (.Quantity (Utilities|Struct|BreakBPS_ItemSlot _array_element)) (CallFunction|GetMaxStackSize ItemID))
        (return _array_index true))))
  (return -1 false))

(fn GetMaxStackSize
  (params (ItemID :type Name))
  (bind _returnvalue (Utilities|GetDataTableRow "/Game/Inventory/Blueprints/DT_ItemData.DT_ItemData" ItemID)
    (:then
      (return (.StackSize (Utilities|Struct|BreakBPS_ItemData _returnvalue))))
    (:RowNotFound
      (return -1))))

(fn AddtoStack
  (params (InventoryIndex :type Integer) (Quantity :type Integer))
  (bind _inventorycontent (Variables|Default|GetInventoryContent))
  (bind _output (Utilities|Array|Get(acopy) _inventorycontent InventoryIndex))
  (Utilities|Array|SetArrayElem _inventorycontent InventoryIndex (Utilities|Struct|MakeBPS_ItemSlot (.itemid _output) (+ (.quantity _output) Quantity))))

(fn AnyEmptySlotsAvailable
  (for (_array_element _array_index) (Variables|Default|GetInventoryContent)
    (if (== (.Quantity (Utilities|Struct|BreakBPS_ItemSlot _array_element)) 0)
      (return true _array_index)))
  (return false -1))

(fn CreateNewStack
  (params (ItemID :type Name) (Quantity :type Integer))
  (bind (_hasemptyslot _emptyindex) (CallFunction|AnyEmptySlotsAvailable))
  (if _hasemptyslot
    (Utilities|Array|SetArrayElem (Variables|Default|GetInventoryContent) _emptyindex (Utilities|Struct|MakeBPS_ItemSlot ItemID Quantity))
    (return true)
    (else
      (return false))))

(fn DebugPrintContent
  (for (_array_element _array_index) (Variables|Default|GetInventoryContent)
    (Development|PrintString (Utilities|String|Append (Utilities|String|ToString(Integer) _array_index) ": " (Utilities|String|ToString(Name) (.ItemID (Utilities|Struct|BreakBPS_ItemSlot _array_element))) " = " (Utilities|String|ToString(Integer) (.Quantity (Utilities|Struct|BreakBPS_ItemSlot _array_element)))))))

(fn ClearInventory
  (Utilities|Array|Clear (Variables|Default|GetInventoryContent))
  (Utilities|Array|Resize (Variables|Default|GetInventoryContent) (Variables|Default|GetInventorySize)))

(fn TransferSlots
  (params (SourceIndex :type Integer) (SourceInventorySystem :type BPC%20Inventory%20Object%20Reference) (DestinationIndex :type Integer))
  (LocalVariables|SetLocalSlotContent (Utilities|Array|Get(acopy) (Variables|BPC_Inventory_C|GetInventoryContent SourceInventorySystem) SourceIndex))
  (if (not (< DestinationIndex 0))
    (if (not (== (.ItemID (Utilities|Struct|BreakBPS_ItemSlot (LocalVariables|GetLocalSlotContent))) (.ItemID (Utilities|Struct|BreakBPS_ItemSlot (Utilities|Array|Get(acopy) (Variables|Default|GetInventoryContent) DestinationIndex)))))
      (Utilities|Array|SetArrayElem (Variables|BPC_Inventory_C|GetInventoryContent SourceInventorySystem) SourceIndex (Utilities|Array|Get(acopy) (Variables|Default|GetInventoryContent) DestinationIndex))
      (Utilities|Array|SetArrayElem (Variables|Default|GetInventoryContent) DestinationIndex (LocalVariables|GetLocalSlotContent))
      (CallFunction|MCUpdate)
      (CallFunction|MCUpdate SourceInventorySystem))))