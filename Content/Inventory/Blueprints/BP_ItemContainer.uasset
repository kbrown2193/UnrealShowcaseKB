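; BP_ItemContainer is an interactable container that shows its InventoryComponent contents on the interacting player's HUD.
; Interact forwards the player character to a local-interact event, which calls DisplayContainer on that player's HudReference.
; An author note flags that the HUD only displays on the server, because Interact is currently called only server-side.
; An unconnected debug branch prints authority and server status but never runs.
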(event Custom|OnLocal_Interact
  (params (Player%20Character :type BP%20First%20Person%20Character%20Object%20Reference))
  ;[1 1 1] Local Interaction - Display Hud - ERROR, ONLY DISPLAY ON SERVER RIGHT NOW, as the event interact is only called server side at the moment
  (Default|DisplayContainer (Variables|/Game/FirstPerson/Blueprints/BP_FirstPersonCharacter.BP_FirstPersonCharacter_C|GetHudReference Player%20Character) (Variables|Default|GetInventoryComponent)))

(event EventInteract
  (params (PlayerCharacter :type BP%20First%20Person%20Character%20Object%20Reference))
  (CallFunction|OnLocalInteract PlayerCharacter))

(fn ConstructionScript)