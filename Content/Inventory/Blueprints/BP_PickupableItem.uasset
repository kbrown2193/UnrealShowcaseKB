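; Replicated world pickup actor for an inventory item, defined by a data table row and quantity in its item data component.
; On BeginPlay it enables replication and sets its static mesh from that row.
; On Interact it adds the row name and quantity to the player's inventory component, destroying itself on success or otherwise keeping the remaining quantity.
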(event EventBeginPlay
  (bind _bpc_itemdata (Variables|Default|GetBPC_ItemData))
  (bind _itemid (Variables|/Game/Inventory/Blueprints/BPC_ItemData.BPC_ItemData_C|GetItemID _bpc_itemdata))
  (Networking|SetReplicates true)
  (bind _returnvalue (Utilities|GetDataTableRow (.datatable _itemid) (.rowname _itemid))
    (:then
      (Components|StaticMesh|SetStaticMesh (Variables|Default|GetItemMesh) (.ItemMesh (Utilities|Struct|BreakBPS_ItemData _returnvalue))))))

(event EventInteract
  (params (PlayerCharacter :type BP%20First%20Person%20Character%20Object%20Reference))
  (bind _bpc_inventory (Variables|/Game/FirstPerson/Blueprints/BP_FirstPersonCharacter.BP_FirstPersonCharacter_C|GetBPC_Inventory PlayerCharacter))
  (bind _bpc_itemdata (Variables|Default|GetBPC_ItemData))
  (bind _bpc_itemdata_2 (Variables|Default|GetBPC_ItemData))
  (bind _itemid (Variables|/Game/Inventory/Blueprints/BPC_ItemData.BPC_ItemData_C|GetItemID _bpc_itemdata_2))
  (bind _returnvalue (Utilities|GetDataTableRow (.datatable _itemid) (.rowname _itemid))
    (:then
      (if (Utilities|IsValid _bpc_inventory)
        (bind (_wassuccessful _quantityremaining) (Default|AddtoInventory _bpc_inventory (.rowname (Variables|/Game/Inventory/Blueprints/BPC_ItemData.BPC_ItemData_C|GetItemID _bpc_itemdata)) (Variables|/Game/Inventory/Blueprints/BPC_ItemData.BPC_ItemData_C|GetQuantity _bpc_itemdata)))
        (if _wassuccessful
          (Actor|DestroyActor)
          (else
            (Variables|/Game/Inventory/Blueprints/BPC_ItemData.BPC_ItemData_C|SetQuantity _bpc_itemdata _quantityremaining)))))))

(fn ConstructionScript)