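; BP_Fridge is a kitchen fridge actor that shows its temperature on a text render component.
; On BeginPlay, a refresh event switches on the temperature's unit (Kelvin, Celsius, Fahrenheit or Rankine) and looks up the matching row in the DT_Units data table.
; The row's unit symbol is formatted with the stored value and written to the text, without any unit conversion.
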(event Custom|RefreshTemperatureDisplayText
  (bind _temperature (Variables|Default|GetTemperature))
  (bind _temperaturetextrender (Variables|Default|GetTemperatureTextRender))
  (switch Utilities|FlowControl|Switch|SwitchonE_Unit_Temperature (.temperatureunit _temperature)
    (:NewEnumerator0
      (bind _returnvalue (Utilities|GetDataTableRow "/Game/Measurement/Units/DT_Units.DT_Units" "Temperature_Kelvin")
        (:then
          (Rendering|Components|TextRender|SetText _temperaturetextrender (Utilities|Text|FormatText "{Value} {Unit}" (.temperaturevalue _temperature) (.UnitSymbol (Utilities|Struct|BreakS_Unit_Definition _returnvalue)))))))
    (:NewEnumerator1
      (bind _returnvalue_2 (Utilities|GetDataTableRow "/Game/Measurement/Units/DT_Units.DT_Units" "Temperature_Celsius")
        (:then
          (Rendering|Components|TextRender|SetText _temperaturetextrender (Utilities|Text|FormatText "{Value} {Unit}" (.temperaturevalue _temperature) (.UnitSymbol (Utilities|Struct|BreakS_Unit_Definition _returnvalue_2)))))))
    (:NewEnumerator2
      (bind _returnvalue_3 (Utilities|GetDataTableRow "/Game/Measurement/Units/DT_Units.DT_Units" "Temperature_Fahrenheit")
        (:then
          (Rendering|Components|TextRender|SetText _temperaturetextrender (Utilities|Text|FormatText "{Value} {Unit}" (.temperaturevalue _temperature) (.UnitSymbol (Utilities|Struct|BreakS_Unit_Definition _returnvalue_3)))))))
    (:NewEnumerator3
      (bind _returnvalue_4 (Utilities|GetDataTableRow "/Game/Measurement/Units/DT_Units.DT_Units" "Temperature_Rankine")
        (:then
          (Rendering|Components|TextRender|SetText _temperaturetextrender (Utilities|Text|FormatText "{Value} {Unit}" (.temperaturevalue _temperature) (.UnitSymbol (Utilities|Struct|BreakS_Unit_Definition _returnvalue_4)))))))))

(event EventBeginPlay
  (CallFunction|RefreshTemperatureDisplayText))

(fn ConstructionScript)