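; BP_Map_SubZone is a map trigger actor that tracks when the player enters or leaves a sub-zone identified by SubZoneID.
; On begin and end overlap, it confirms the other actor is player 0's pawn and casts it to BP_FirstPersonCharacter.
; It then prints a debug message and passes the ID to the character's EnterSubzone or ExitSubzone, leaving any zone response to the character.
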(event Collision|EventActorBeginOverlap
  (params (OtherActor :type Actor%20Object%20Reference))
  (if (== OtherActor (Game|Player|GetPlayerPawn 0))
    (bind _asbp_first_person_character (Utilities|Casting|CastToBP_FirstPersonCharacter OtherActor))
    (Development|PrintString (Utilities|String|Append "MSZ: Player detected entering zone " (Utilities|String|ToString(Name) (Variables|Default|GetSubZoneID))))
    (Default|EnterSubzone _asbp_first_person_character (Variables|Default|GetSubZoneID))))

(event Collision|EventActorEndOverlap
  (params (OtherActor :type Actor%20Object%20Reference))
  (if (== OtherActor (Game|Player|GetPlayerPawn 0))
    (bind _asbp_first_person_character (Utilities|Casting|CastToBP_FirstPersonCharacter OtherActor))
    (Development|PrintString (Utilities|String|Append "MSZ: Player detected exiting  zone " (Utilities|String|ToString(Name) (Variables|Default|GetSubZoneID))))
    (Default|ExitSubzone _asbp_first_person_character (Variables|Default|GetSubZoneID))))

(fn ConstructionScript)