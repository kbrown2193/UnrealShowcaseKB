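; BP_Map_Zone is a map zone actor that tells the first-person player character when it enters or leaves the zone identified by ZoneID.
; Begin and end overlap events filter for player 0's pawn, cast it to BP_FirstPersonCharacter, and call its EnterZone or ExitZone with that ID.
; Both events also print a debug message, and the zone logic itself is left to the character.
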(event Collision|EventActorBeginOverlap
  (params (OtherActor :type Actor%20Object%20Reference))
  (if (== OtherActor (Game|Player|GetPlayerPawn 0))
    (bind _asbp_first_person_character (Utilities|Casting|CastToBP_FirstPersonCharacter OtherActor))
    (Development|PrintString (Utilities|String|Append "MZ: Player detected entering zone " (Utilities|String|ToString(Name) (Variables|Default|GetZoneID))))
    (Default|EnterZone _asbp_first_person_character (Variables|Default|GetZoneID))))

(event Collision|EventActorEndOverlap
  (params (OtherActor :type Actor%20Object%20Reference))
  (if (== OtherActor (Game|Player|GetPlayerPawn 0))
    (bind _asbp_first_person_character (Utilities|Casting|CastToBP_FirstPersonCharacter OtherActor))
    (Development|PrintString (Utilities|String|Append "MZ: Player detected exiting  zone " (Utilities|String|ToString(Name) (Variables|Default|GetZoneID))))
    (Default|ExitZone _asbp_first_person_character (Variables|Default|GetZoneID))))

(fn ConstructionScript)