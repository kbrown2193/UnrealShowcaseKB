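; BP_MusicPlayer plays background music on its MusicAudio component, chosen by song ID or map zone ID.
; Play events look up DT_Music or DT_Zones, set the sound and fade it in.
; Single-track zones skip a track already set and bind a finish handler that replays it when IsLooping is set.
; Multi-track zones pick the first listed track differing from the current one, without binding a finish handler.
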(event Custom|PlayMusicViaSongID
  (params (SongID :type Name))
  (bind _music_audio (Variables|Default|GetMusic_Audio))
  (bind _returnvalue (Utilities|GetDataTableRow "/Game/Music/DataTables/DT_Music.DT_Music" SongID)
    (:then
      (Audio|Components|Audio|SetSound _music_audio (.SoundWave (Utilities|Struct|BreakS_Music _returnvalue)))
      (Audio|Components|Audio|FadeIn _music_audio 2.0 1.0 0.0 "Linear" :!class /Script/Engine.AudioComponent))
    (:RowNotFound
      (Development|PrintString "Song not found in Music data table" true true "(R=1.000000,G=0.000000,B=0.010000,A=1.000000)"))))

(event Custom|PlayMusicViaZoneIDSingleTrack
  (params (ZoneID :type Name))
  (bind _music_audio (Variables|Default|GetMusic_Audio))
  (bind _music_audio_2 (Variables|Default|GetMusic_Audio))
  (bind _returnvalue (Utilities|GetDataTableRow "/Game/Map/DataTables/DT_Zones.DT_Zones" ZoneID)
    (:then
      (Utilities|IsValid (.MusicTrack (Utilities|Struct|BreakS_Zone _returnvalue))
        (:Is%20Valid
          (if (not (== (.MusicTrack (Utilities|Struct|BreakS_Zone _returnvalue)) (Variables|/Script/Engine.AudioComponent|GetSound _music_audio)))
            (Audio|Components|Audio|SetSound _music_audio (.MusicTrack (Utilities|Struct|BreakS_Zone _returnvalue)))
            (Audio|Components|Audio|FadeIn _music_audio_2 2.0 1.0 0.0 "Linear" :!class /Script/Engine.AudioComponent)
            (if (Variables|Default|GetIsLooping)
              (EventDispatchers|BindEventtoOnAudioFinished _music_audio_2 (delegate Custom|SongEndLoop))
              (else
                (EventDispatchers|BindEventtoOnAudioFinished _music_audio_2 (delegate Custom|SongEndNotLoop))))
            (else
              (Development|PrintString "Already Playing song"))))
        (:Is%20Not%20Valid
          (Development|PrintString "No song specified in Map Zones data table" true true "(R=0.974000,G=0.000000,B=0.005000,A=1.000000)"))))))

(event Custom|PlayMusicViaZoneIDMultipleTracks
  (params (ZoneID :type Name))
  (bind _music_audio (Variables|Default|GetMusic_Audio))
  (bind _returnvalue (Utilities|GetDataTableRow "/Game/Map/DataTables/DT_Zones.DT_Zones" ZoneID)
    (:then
      (bind _array_element (Utilities|Array|ForEachLoopwithBreak (.MusicTracks (Utilities|Struct|BreakS_Zone _returnvalue)) :!label _label)
        (:LoopBody
          (if (not (== _array_element (Variables|/Script/Engine.AudioComponent|GetSound _music_audio)))
            (Audio|Components|Audio|SetSound _music_audio _array_element)
            (goto _label Break)))
        (:Completed
          (Audio|Components|Audio|FadeIn (Variables|Default|GetMusic_Audio) 0.0 1.0 0.0 "Linear" :!class /Script/Engine.AudioComponent))))))

(event Custom|SongEndNotLoop
  (Development|PrintString "Music Player Finished song,"))

(event Custom|SongEndLoop
  (Development|PrintString "Music Player Finished song, Looping")
  (Audio|Components|Audio|FadeIn (Variables|Default|GetMusic_Audio) 2.0 1.0 0.0 "Linear" :!class /Script/Engine.AudioComponent))

(fn ConstructionScript)