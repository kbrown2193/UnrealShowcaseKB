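; BP_SoundSystemController is a music playlist controller that keeps a set of sound speakers on the same current song.
; On BeginPlay it loops over SoundSpeakers, setting and playing the SongList entry at CurrentSong on each.
; SongEnd advances the index and replays on all speakers, wrapping to zero, though its bounds check lets the index step one past the last song.
; SetAllSpeakerSounds assigns the current song without playing it.
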(event Custom|SetAllSpeakerSounds
  (for _array_element (Variables|Default|GetSoundSpeakers)
    (Default|SetSound _array_element (Utilities|Array|Get(acopy) (Variables|Default|GetSongList) (Variables|Default|GetCurrentSong)))))

(event Custom|SetAllSpeakerSoundsAndPlay
  (for _array_element (Variables|Default|GetSoundSpeakers)
    (Default|SetandPlaySound _array_element (Utilities|Array|Get(acopy) (Variables|Default|GetSongList) (Variables|Default|GetCurrentSong)))))

(event Custom|SongEnd
  (if (< (Variables|Default|GetCurrentSong) (Utilities|Array|Length (Variables|Default|GetSongList)))
    (Math|Integer|IncrementInt (Variables|Default|GetCurrentSong)
      (:%20%20
        (CallFunction|SetAllSpeakerSoundsandPlay)))
    (else
      (Variables|Default|SetCurrentSong 0)
      (CallFunction|SetAllSpeakerSoundsandPlay))))

(event EventBeginPlay
  (CallFunction|SetAllSpeakerSoundsandPlay))

(fn ConstructionScript)