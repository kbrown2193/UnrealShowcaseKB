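; Bass drum pedal Blueprint that animates the swing of its beater.
; BeginPlay sets the beater root's roll to the negated resting angle and prints a todo about default pedal setup.
; PressPedal restarts a timeline whose curve scales that negated angle, adds the resting angle, and applies the result as the beater root's roll.
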(event Custom|PressPedal
  (bind _beaterrotation (Timeline|PedalRotation PlayFromStart)
    (:Update
      (Transformation|SetRelativeRotation (Variables|Default|GetBeaterRotationRoot) (Math|Rotator|MakeRotator (+ (* _beaterrotation (Variables|Default|GetBeaterRotationAngle)) (Variables|Default|GetRestingAngle)) 0.0 0.0) false false))))

(event Custom|InitializeStartingPositions
  (bind _output_get (Variables|Default|SetBeaterRotationAngle (* (Variables|Default|GetRestingAngle) -1.0)))
  (Transformation|SetRelativeRotation (Variables|Default|GetBeaterRotationRoot) (Math|Rotator|MakeRotator _output_get 0.0 0.0) false false))

(event EventBeginPlay
  (Development|PrintString "todo: set default pedal setup")
  (CallFunction|InitializeStartingPositions))

(fn ConstructionScript)