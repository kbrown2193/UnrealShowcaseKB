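; Drumset instrument actor with events to play its closed hi-hat, bass drum and snare.
; Each event plays its sound at the matching drum mesh, gated by the IsPlayingSound flag.
; The hi-hat also runs a timeline that tilts both cymbal meshes, and the bass drum presses a child-actor pedal, even when sound is off.
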(event Custom|PlayHiHatClosed
  (bind _sm_drum_hihat_14in_1mm_bot (Variables|Default|GetSM_Drum_HiHat_14in_1mm_Bot))
  (bind _sm_drum_hihat_14in_1mm_top (Variables|Default|GetSM_Drum_HiHat_14in_1mm_Top))
  (bind _relativerotation (Variables|/Script/Engine.SceneComponent|GetRelativeRotation _sm_drum_hihat_14in_1mm_top))
  (bind _relativerotation_2 (Variables|/Script/Engine.SceneComponent|GetRelativeRotation _sm_drum_hihat_14in_1mm_bot))
  (bind (_roll _pitch _yaw) (Math|Rotator|BreakRotator _relativerotation))
  (bind (_roll_2 _pitch_2 _yaw_2) (Math|Rotator|BreakRotator _relativerotation_2))
  (if (Variables|Default|GetIsPlayingSound)
    (Audio|PlaySoundatLocation "/Game/Music/Cues/SC_Drumset_HiHat.SC_Drumset_HiHat" (Transformation|GetWorldLocation (Variables|Default|GetSM_Drum_HiHat_14in_1mm_Top)) "0, 0, 0" 1.0 1.0 0.0 0 0 0 0)
    (bind _rotytrack (Timeline|HiHatPlayTimeline PlayFromStart)
      (:Update
        (Transformation|SetRelativeRotation _sm_drum_hihat_14in_1mm_top (Math|Rotator|MakeRotator _roll _rotytrack _yaw) false false)
        (Transformation|SetRelativeRotation _sm_drum_hihat_14in_1mm_bot (Math|Rotator|MakeRotator _roll_2 _rotytrack _yaw_2) false false)))
    (else
      (Timeline|HiHatPlayTimeline PlayFromStart))))

(event Custom|BassDrumPlay
  (Default|PressPedal (.AsBP%20Bassdrum%20Pedal (Utilities|Casting|CastToBP_Bassdrum_Pedal (Variables|/Script/Engine.ChildActorComponent|GetChildActor (Variables|Default|GetBP_Bassdrum_Pedal)))))
  (if (Variables|Default|GetIsPlayingSound)
    (Audio|PlaySoundatLocation "/Game/Music/Cues/SC_Drumset_BassDrum.SC_Drumset_BassDrum" (Transformation|GetWorldLocation (Variables|Default|GetSM_Drum_Bass_22DIA_18DEP_inches_v01e00)) "0, 0, 0" 1.0 1.0 0.0 0 0 0 0)))

(event Custom|SnareDrumPlay
  (if (Variables|Default|GetIsPlayingSound)
    (Audio|PlaySoundatLocation "/Game/Music/Cues/SC_Drumset_SnareDrum.SC_Drumset_SnareDrum" (Transformation|GetWorldLocation (Variables|Default|GetSM_Drum_Snare_14DIA_6p5DEP_inches_v01e00)) "0, 0, 0" 1.0 1.0 0.0 0 0 0 0)))

(event EventBeginPlay)

(event Collision|EventActorBeginOverlap
  (params (OtherActor :type Actor%20Object%20Reference)))

(event EventTick
  (params (DeltaSeconds :type Float%20%28single-precision%29)))

(fn ConstructionScript)