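; BP_NPC_00 is an interactable NPC that shows a dialog box to the player.
; On Interact it prints a greeting, creates and displays a W_DialogBox widget if none exists, then fills its text with a random integer as placeholder dialog.
; When the player character leaves TriggerZone, it removes the widget and clears the reference.
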(event OnComponentEndOverlap(TriggerZone)
  (params (OverlappedComponent :type Primitive%20Component%20Object%20Reference) (OtherActor :type Actor%20Object%20Reference) (OtherComp :type Primitive%20Component%20Object%20Reference) (OtherBodyIndex :type Integer))
  (if (== OtherActor (Game|GetPlayerCharacter 0))
    (bind _dialogboxui (Variables|Default|GetDialogBoxUI)
      (:then
        (Widget|RemovefromParent _dialogboxui)
        (Variables|Default|SetDialogBoxUI 0))
      (:else))))

(event EventInteract
  (params (PlayerCharacter :type BP%20First%20Person%20Character%20Object%20Reference))
  (Development|PrintString "Hello")
  (Variables|Default|GetDialogBoxUI
    (:then
      _)
    (:else
      (bind _returnvalue (UserInterface|CreateWidget "/Game/Dialog/UI/W_DialogBox.W_DialogBox_C" (Game|GetPlayerController 0)))
      (bind _output_get (Variables|Default|SetDialogBoxUI _returnvalue))
      (UserInterface|Viewport|AddtoViewport _output_get 0)))
  (Variables|/Script/UMG.TextBlock|SetText (Variables|/Game/Dialog/UI/W_DialogBox.W_DialogBox_C|GetDialogText (Variables|Default|GetDialogBoxUI)) (Utilities|Text|ToText(Integer) (Math|Random|RandomInteger 256))))

(fn ConstructionScript)