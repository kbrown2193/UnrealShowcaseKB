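; BP_SaveGameCatalog is a save object that keeps the list of save game slot names.
; Adding a name rejects duplicates, saves the catalog itself to the fixed "SaveGameCatalog" slot on success, and returns whether the name was added.
; Removing a name only edits the array in memory and does not write the catalog to disk.
; Both functions report their results through debug prints.
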(fn AddSaveGametoNames
  (params (NewSaveGameName :type String))
  (bind _savegameslotnames (Variables|Default|GetSaveGameSlotNames))
  (Variables|Default|SetDoesAlreadyExist false)
  (for _array_element _savegameslotnames
    (if (Utilities|Enum|Equal(Enum) NewSaveGameName _array_element)
      (Development|PrintString 0 "SAVE GAME NAME ALREADY EXISTS")
      (Variables|Default|SetDoesAlreadyExist true)))
  (Development|PrintString 0 "Loop Completed")
  (if (Variables|Default|GetDoesAlreadyExist)
    _
    (else
      (Utilities|Array|Add _savegameslotnames NewSaveGameName)
      (Development|PrintString 0 (Utilities|String|Append NewSaveGameName " Added to save game slot names"))
      (SaveGame|SaveGametoSlot self "SaveGameCatalog")
      (Development|PrintString 0 "SaveGameCatalog Saved")))
  (return (not (Variables|Default|GetDoesAlreadyExist))))

(fn RemoveSaveGameName
  (params (SaveGameNameToRemove :type String))
  (bind _savegameslotnames (Variables|Default|GetSaveGameSlotNames))
  (if (Utilities|Array|ContainsItem _savegameslotnames SaveGameNameToRemove)
    (Utilities|Array|RemoveItem _savegameslotnames SaveGameNameToRemove)
    (Development|PrintString 0 (Utilities|String|Append SaveGameNameToRemove " Removed from save game catalog"))
    (else
      (Development|PrintString 0 "COULD NOT FIND SAVE GAME"))))