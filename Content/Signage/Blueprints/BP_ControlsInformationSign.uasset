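; In-world sign Blueprint intended to show key bindings for move, look, jump, interact, flashlight and inventory on a text render.
; GetKeyDisplayName queries Enhanced Input for each action's mapped keys, printing debug output.
; It returns the first key for mouse-and-keyboard controls, otherwise the first 2D-axis or gamepad key, falling back to "Not Found".
; The text update is disconnected from the empty BeginPlay pending a working lookup, so the sign never updates.
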(event EventBeginPlay
  ;[1 1 1] TODO: Connect when GetKeyDisplayName works
)

(fn ConstructionScript)

(fn GetKeyDisplayName
  (params (IA :type Input%20Action%20Object%20Reference))
  (bind _returnvalue (Class|EnhancedInputSubsystemInterface|QueryKeysMappedtoAction(Message) (PlayerController|LocalPlayerSubsystems|GetEnhancedInputLocalPlayerSubsystem) IA))
  (Development|PrintString (Utilities|String|BuildString(Integer) (Utilities|String|Append "Action Count for " (Utilities|GetDisplayName IA)) " =  " (Utilities|Array|Length _returnvalue)) true true "(R=1.000000,G=0.942108,B=0.372747,A=1.000000)" 2e+01)
  (for (_array_element _array_index) _returnvalue
    (Development|PrintString (Utilities|String|Append (Utilities|String|ToString(Integer) _array_index) (Utilities|String|ToString(Text) (Class|KismetInputLibrary|KeyGetDisplayName _array_element true))) true true "(R=0.000000,G=1.000000,B=0.210418,A=1.000000)" 2e+01)
    (if (Variables|Default|GetIsMouseAndKeyboardControls)
      (return (Class|KismetInputLibrary|KeyGetDisplayName _array_element true))
      (elif (Class|KismetInputLibrary|KeyIsAxis2D _array_element)
        (if true
          (return (Class|KismetInputLibrary|KeyGetDisplayName _array_element true)))
        (elif (Class|KismetInputLibrary|KeyIsGamepadKey _array_element)
          (return (Class|KismetInputLibrary|KeyGetDisplayName _array_element true))))))
  (return "Not Found"))