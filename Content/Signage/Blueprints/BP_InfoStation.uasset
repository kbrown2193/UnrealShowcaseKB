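; BP_InfoStation is an information sign actor that shows its location as text alongside world, city and zone maps.
; On BeginPlay it chains Data Table lookups by world, city, zone and subzone ID, then writes the names to a text render.
; It applies each row's map material to the matching plane.
; A missing subzone drops that line, while other missing rows only print an error.
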(event EventBeginPlay
  (bind _returnvalue (Utilities|String|Append " 
" ""))
  (bind _infostation_map_textrender (Variables|Default|GetInfostation_Map_TextRender))
  (bind _returnvalue_2 (Utilities|GetDataTableRow "/Game/Map/DataTables/DT_Worlds.DT_Worlds" (Variables|Default|GetWorldID))
    (:then
      (bind _returnvalue_3 (Utilities|GetDataTableRow "/Game/Map/DataTables/DT_Cities.DT_Cities" (Variables|Default|GetCityID))
        (:then
          (bind _returnvalue_4 (Utilities|GetDataTableRow "/Game/Map/DataTables/DT_Zones.DT_Zones" (Variables|Default|GetZoneID))
            (:then
              (bind _returnvalue_5 (Utilities|GetDataTableRow "/Game/Map/DataTables/DT_Subzones.DT_Subzones" (Variables|Default|GetSubzoneID))
                (:then
                  (Rendering|Components|TextRender|SetText _infostation_map_textrender (Utilities|Text|FormatText "{World}{LineBreak}{City}{LineBreak}{ Zone}{LineBreak}{Subzone}" (Utilities|Text|ToText(Name) (.WorldName (Utilities|Struct|BreakS_World _returnvalue_2))) _returnvalue (Utilities|Text|ToText(Name) (.CityName (Utilities|Struct|BreakS_City _returnvalue_3))) (Utilities|Text|ToText(Name) (.ZoneName (Utilities|Struct|BreakS_Zone _returnvalue_4))) (Utilities|Text|ToText(Name) (Utilities|Struct|BreakS_SubZone _returnvalue_5)))))
                (:RowNotFound
                  (Development|PrintString "InfoStation. SubZone not found" true true "(R=1.000000,G=0.947000,B=0.010000,A=1.000000)")
                  (Rendering|Components|TextRender|SetText _infostation_map_textrender (Utilities|Text|FormatText "{World}{LineBreak}{City}{LineBreak}{ Zone}" (Utilities|Text|ToText(Name) (.WorldName (Utilities|Struct|BreakS_World _returnvalue_2))) _returnvalue (Utilities|Text|ToText(Name) (.CityName (Utilities|Struct|BreakS_City _returnvalue_3))) (Utilities|Text|ToText(Name) (.ZoneName (Utilities|Struct|BreakS_Zone _returnvalue_4)))))))
              (Rendering|Material|SetMaterial (Variables|Default|GetWorldMapPlane) 0 (.WorldMapMaterial (Utilities|Struct|BreakS_World _returnvalue_2)))
              (Rendering|Material|SetMaterial (Variables|Default|GetCityMapPlane) 0 (.CityMapMaterial (Utilities|Struct|BreakS_City _returnvalue_3)))
              (Rendering|Material|SetMaterial (Variables|Default|GetZoneMapPlane) 0 (.ZoneMapMaterial (Utilities|Struct|BreakS_Zone _returnvalue_4))))
            (:RowNotFound
              (Development|PrintString "InfoStation. Zone not found" true true "(R=1.000000,G=0.947000,B=0.010000,A=1.000000)"))))
        (:RowNotFound
          (Development|PrintString "InfoStation. City not found" true true "(R=1.000000,G=0.947000,B=0.010000,A=1.000000)"))))
    (:RowNotFound
      (Development|PrintString "InfoStation. World not found" true true "(R=1.000000,G=0.947000,B=0.010000,A=1.000000)"))))

(fn ConstructionScript)