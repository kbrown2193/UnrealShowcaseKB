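; BP_OpenSign is a signage actor for an open sign that switches between lit and unlit looks.
; TurnOn and TurnOff set the IsOn flag and swap the sign mesh's first material slot between the On and Off material instances.
; BeginPlay applies the initial IsOn state, and ToggleOnOff flips it.
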(event EventBeginPlay
  (if (Variables|Default|GetIsOn)
    (CallFunction|Turnon)
    (else
      (CallFunction|TurnOff))))

(event Collision|EventActorBeginOverlap
  (params (OtherActor :type Actor%20Object%20Reference)))

(event EventTick
  (params (DeltaSeconds :type Float%20%28single-precision%29)))

(fn ConstructionScript)

(fn Turnon
  (Variables|Default|SetIsOn true)
  (Rendering|Material|SetMaterial (Variables|Default|GetOpenSign_Mesh) 0 "/Game/Signage/Mesh/MI_OpenSign_On.MI_OpenSign_On"))

(fn TurnOff
  (Variables|Default|SetIsOn false)
  (Rendering|Material|SetMaterial (Variables|Default|GetOpenSign_Mesh) 0 "/Game/Signage/Mesh/MI_OpenSign_Off.MI_OpenSign_Off"))

(fn ToggleonOff
  (if (Variables|Default|GetIsOn)
    (CallFunction|TurnOff)
    (else
      (CallFunction|Turnon))))