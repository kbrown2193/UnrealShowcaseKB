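; BP_Planet is a planet actor that spins a sphere on a tilted axis, configured by a DT_Planets row keyed by PlanetID.
; The row sets scale, day length, axial tilt and an optional detail texture through a dynamic M_Planet material.
; BeginPlay optionally loads the row, then starts a self-restarting timeline whose rate derives from day length and a time multiplier.
; InitializePlanet applies a given ID's row, but without EarthSizeScaler or a play-rate update.
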(event Custom|PlanetRotationLoop
  (bind _fullrotationangle (Timeline|PlanetRotationTimeline PlayFromStart)
    (:Update
      (Transformation|SetRelativeRotation (Variables|Default|GetPlanet_Sphere) (Math|Rotator|MakeRotator 0.0 (Variables|Default|GetAxialTilt) (* _fullrotationangle -1.0)) false false))
    (:Finished
      (CallFunction|PlanetRotationLoop))))

(event EventBeginPlay
  (if (Variables|Default|GetIsDataTablePlanet)
    (CallFunction|SetVariablesfromPlanetsDataTable)
    (else
      (Development|PrintString "Not Data Table Planet")))
  (Components|Timeline|SetPlayRate (Variables|Default|GetPlanetRotationTimeline) (* (/ 1.0 (Variables|Default|GetDurationOfRotation)) (Variables|Default|GetRealTimeScaleMultiplier)))
  (CallFunction|PlanetRotationLoop))

(fn ConstructionScript)

(fn SetVariablesfromPlanetsDataTable
  (bind _planetid (Variables|Default|GetPlanetID))
  (bind _returnvalue (Utilities|GetDataTableRow "/Game/Space/Data/DT_Planets.DT_Planets" _planetid)
    (:then
      (Transformation|SetRelativeScale3D (Variables|Default|GetPlanet_Sphere) (Math|Conversions|ToVector(Float) (* (.Size (Utilities|Struct|BreakS_Planet _returnvalue)) (Variables|Default|GetEarthSizeScaler))))
      (Variables|Default|SetDurationOfRotation (.LengthOfDay (Utilities|Struct|BreakS_Planet _returnvalue)))
      (Variables|Default|SetAxialTilt (.AxialTilt (Utilities|Struct|BreakS_Planet _returnvalue)))
      (if (Utilities|IsValid (.DetailTexture (Utilities|Struct|BreakS_Planet _returnvalue)))
        (bind _returnvalue_2 (Rendering|Material|CreateDynamicMaterialInstance (Variables|Default|GetPlanet_Sphere) 0 "/Game/Space/Materials/M_Planet.M_Planet" "None" :!class /Script/Engine.PrimitiveComponent))
        (Rendering|Material|SetTextureParameterValue _returnvalue_2 "PlanetDetailTexture" (.DetailTexture (Utilities|Struct|BreakS_Planet _returnvalue)))))
    (:RowNotFound
      (Development|PrintString (Utilities|String|Append (Utilities|String|ToString(Name) _planetid) "NOT FOUND") true true "(R=1.000000,G=0.000000,B=0.000000,A=1.000000)"))))

(fn InitializePlanet
  (params (NewPlanetID :type Name))
  (bind _output_get (Variables|Default|SetPlanetID NewPlanetID))
  (bind _returnvalue (Utilities|GetDataTableRow "/Game/Space/Data/DT_Planets.DT_Planets" _output_get)
    (:then
      (Transformation|SetRelativeScale3D (Variables|Default|GetPlanet_Sphere) (Math|Conversions|ToVector(Float) (.Size (Utilities|Struct|BreakS_Planet _returnvalue))))
      (Variables|Default|SetDurationOfRotation (.LengthOfDay (Utilities|Struct|BreakS_Planet _returnvalue)))
      (Variables|Default|SetAxialTilt (.AxialTilt (Utilities|Struct|BreakS_Planet _returnvalue)))
      (if (Utilities|IsValid (.DetailTexture (Utilities|Struct|BreakS_Planet _returnvalue)))
        (bind _returnvalue_2 (Rendering|Material|CreateDynamicMaterialInstance (Variables|Default|GetPlanet_Sphere) 0 "/Game/Space/Materials/M_Planet.M_Planet" "None" :!class /Script/Engine.PrimitiveComponent))
        (Rendering|Material|SetTextureParameterValue _returnvalue_2 "PlanetDetailTexture" (.DetailTexture (Utilities|Struct|BreakS_Planet _returnvalue)))))
    (:RowNotFound
      (Development|PrintString (Utilities|String|Append "" "NOT FOUND") true true "(R=1.000000,G=0.000000,B=0.000000,A=1.000000)"))))