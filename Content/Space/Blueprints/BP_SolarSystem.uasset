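; BP_SolarSystem is an actor that builds a solar system from a DT_SolarSystems data table row.
; InitializeSolarSystem looks up the ID, sets the name text render, then passes the row's star and planet IDs to their initializers.
; InitializeStars spawns and initializes BP_Star actors at this actor's transform.
; Multi-star relative placement is still a TODO, and InitializePlanets is an empty stub.
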(event EventBeginPlay)

(event Collision|EventActorBeginOverlap
  (params (OtherActor :type Actor%20Object%20Reference)))

(event EventTick
  (params (DeltaSeconds :type Float%20%28single-precision%29)))

(fn ConstructionScript)

(fn InitializeSolarSystem
  (params (SolarSystemID :type Name))
  (bind _returnvalue (Utilities|GetDataTableRow "/Game/Space/Data/DT_SolarSystems.DT_SolarSystems" SolarSystemID)
    (:then
      (Rendering|Components|TextRender|SetText (Variables|Default|GetSolarSystemName_TextRender) (Utilities|Text|ToText(Name) (.SolarSystemName (Utilities|Struct|BreakS_SolarSystem _returnvalue))))
      (CallFunction|InitializeStars (.StarIDs (Utilities|Struct|BreakS_SolarSystem _returnvalue)))
      (CallFunction|InitializePlanets (.PlanetIDs (Utilities|Struct|BreakS_SolarSystem _returnvalue)))
      (Development|PrintString (Utilities|String|Append (Utilities|String|ToString(Text) (Utilities|Text|ToText(Name) (.SolarSystemName (Utilities|Struct|BreakS_SolarSystem _returnvalue)))) "solar system initialized") true true "(R=1.000000,G=0.275073,B=0.000000,A=1.000000)" 16.0))))

(fn InitializeStars
  (params (StarIDs :type Array%20of%20Names))
  (if true
    (if (> (Utilities|Array|Length StarIDs) 1)
      (Development|PrintString "Multi star solar system TODO:")
      (for _array_element StarIDs
        (bind _returnvalue (Utilities|GetDataTableRow "/Game/Space/Data/DT_Stars.DT_Stars" _array_element)
          (:then
            (Development|PrintString "TODO: Relative spawning check")
            (bind _returnvalue_2 (Game|SpawnActorfromClass "/Game/Space/Blueprints/BP_Star.BP_Star_C" (Transformation|GetActorTransform) "Undefined" "MultiplyWithRoot" 0 0))
            (Default|InitializeStar _returnvalue_2 _array_element))))
      (else
        (bind _returnvalue_3 (Game|SpawnActorfromClass "/Game/Space/Blueprints/BP_Star.BP_Star_C" (Transformation|GetActorTransform) "Undefined" "MultiplyWithRoot" 0 0))
        (Default|InitializeStar _returnvalue_3 (Utilities|Array|Get(acopy) StarIDs))))))

(fn InitializePlanets
  (params (PlanetIDs :type Array%20of%20Names)))