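; Spawner actor that populates space with a BP_SolarSystem for every row in DT_SolarSystems at BeginPlay.
; Each spawned system is initialized with its row name, with debug prints tracking progress.
; ConvertCoordinatesToTransform turns right ascension, declination and distance into location and rotation using trigonometry, scaled by SpawnDistanceMultiplier.
; The Y component omits the declination cosine, so placement is not a true spherical projection.
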(event EventBeginPlay
  (Development|PrintString "Solar System Spawnwer Started" true true "(R=0.356000,G=0.000000,B=0.005000,A=1.000000)")
  (bind _outrownames (DataTable|GetDataTableRowNames "/Game/Space/Data/DT_SolarSystems.DT_SolarSystems"))
  (for (_array_element _array_index) _outrownames
    (Development|PrintString (Utilities|String|Append (Utilities|String|ToString(Name) _array_element) (Utilities|String|ToString(Integer) _array_index)))
    (bind _returnvalue (Utilities|GetDataTableRow "/Game/Space/Data/DT_SolarSystems.DT_SolarSystems" _array_element)
      (:then
        (bind _spawntransform (CallFunction|ConvertCoordinatestoTransform (.RightAscension (Utilities|Struct|BreakS_CelestialCoordinates (.CelestialCoordinates (Utilities|Struct|BreakS_SolarSystem _returnvalue)))) (.Declination (Utilities|Struct|BreakS_CelestialCoordinates (.CelestialCoordinates (Utilities|Struct|BreakS_SolarSystem _returnvalue)))) (.Distance (Utilities|Struct|BreakS_SolarSystem _returnvalue))))
        (bind _returnvalue_2 (Game|SpawnActorfromClass "/Game/Space/Blueprints/BP_SolarSystem.BP_SolarSystem_C" _spawntransform "Undefined" "MultiplyWithRoot" 0 0))
        (Default|InitializeSolarSystem _returnvalue_2 _array_element))))
  (Development|PrintString "Solar System Spawner Done" true true "(R=0.000000,G=1.000000,B=0.000000,A=1.000000)"))

(event Collision|EventActorBeginOverlap
  (params (OtherActor :type Actor%20Object%20Reference)))

(event EventTick
  (params (DeltaSeconds :type Float%20%28single-precision%29)))

(fn ConstructionScript)

(fn ConvertCoordinatestoTransform
  (params (RightAscension :type S%20Right%20Ascension%20Structure) (Declination :type S%20Declination%20Structure) (Distance :type Float%20%28double-precision%29))
  (bind (_degrees _minutes _seconds _microseconds) (Utilities|Struct|BreakS_Declination Declination))
  (bind (_hours _minutes_2 _seconds_2 _microseconds_2) (Utilities|Struct|BreakS_RightAscension RightAscension))
  (bind _returnvalue (Math|Conversions|ToFloat(Integer) _minutes_2))
  (bind _returnvalue_2 (Math|Conversions|ToFloat(Integer) _seconds_2))
  (bind _returnvalue_3 (Math|Conversions|ToFloat(Integer) _microseconds_2))
  (bind _returnvalue_4 (Math|Conversions|ToFloat(Integer) _degrees))
  (bind _returnvalue_5 (Math|Conversions|ToFloat(Integer) _minutes))
  (bind _returnvalue_6 (Math|Conversions|ToFloat(Integer) _seconds))
  (bind _returnvalue_7 (Math|Conversions|ToFloat(Integer) _microseconds))
  (bind _returnvalue_8 (Math|Conversions|ToFloat(Integer) _hours))
  (bind _returnvalue_9 (/ _returnvalue 6e+01))
  (bind _returnvalue_10 (/ _returnvalue_2 3.6e+03))
  (bind _returnvalue_11 (* _returnvalue_3 1e-06))
  (bind _returnvalue_12 (* _returnvalue_8 15.0))
  (bind _returnvalue_13 (/ _returnvalue_5 6e+01))
  (bind _returnvalue_14 (/ _returnvalue_6 3.6e+03))
  (bind _returnvalue_15 (* _returnvalue_7 1e-06))
  (bind _returnvalue_16 (+ _returnvalue_12 _returnvalue_9 _returnvalue_10 _returnvalue_11))
  (bind _returnvalue_17 (+ _returnvalue_4 _returnvalue_13 _returnvalue_14 _returnvalue_15))
  (return (Math|Transform|MakeTransform (* (Math|Vector|MakeVector (* (Math|Trig|Cos(Degrees) _returnvalue_16) (Math|Trig|Cos(Degrees) _returnvalue_17)) (* (Math|Trig|Sin(Degrees) _returnvalue_16) -1.0) (Math|Trig|Sin(Degrees) _returnvalue_17)) (* Distance (Variables|Default|GetSpawnDistanceMultiplier))) (Math|Rotator|MakeRotator 0.0 (* _returnvalue_17 1.0) (* _returnvalue_16 -1.0)))))