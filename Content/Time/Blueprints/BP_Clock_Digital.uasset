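; BP_Clock_Digital is a digital clock actor that shows a supplied time on its ClockTextRender text component.
; SetTime formats hours and minutes as two-digit values, subtracting 12 from hours above 12 when Is12HourFormat is set, with no AM/PM marker.
; SetTextColor changes the display color.
; The clock has no update logic of its own, so the display changes only when these functions are called.
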(event EventBeginPlay)

(event Collision|EventActorBeginOverlap
  (params (OtherActor :type Actor%20Object%20Reference)))

(event EventTick
  (params (DeltaSeconds :type Float%20%28single-precision%29)))

(fn ConstructionScript)

(fn SetTime
  (params (Hours :type Float%20%28double-precision%29) (Minutes :type Float%20%28double-precision%29))
  (bind _returnvalue (Utilities|Text|ToText(Float) Minutes "HalfToEven" false true 2 2 0 0))
  (bind _clock_textrender (Variables|Default|GetClock_TextRender))
  (if (Variables|Default|GetIs12HourFormat)
    (if (> Hours 12)
      (Rendering|Components|TextRender|SetText _clock_textrender (Utilities|Text|FormatText "{Hours} : {Minutes}" (Utilities|Text|ToText(Float) (- Hours 12.0) "HalfToEven" false true 2 2 0 0) _returnvalue))
      (else
        (Rendering|Components|TextRender|SetText _clock_textrender (Utilities|Text|FormatText "{Hours} : {Minutes}" (Utilities|Text|ToText(Float) Hours "HalfToEven" false true 2 2 0 0) _returnvalue) :!label _label)))
    (else
      (goto _label))))

(fn SetTextColor
  (params (NewTextColor :type Color%20Structure))
  (Rendering|Components|TextRender|SetTextRenderColor (Variables|Default|GetClock_TextRender) NewTextColor))