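; BP_GameTimeManager is an in-game clock and calendar that tracks seconds through years, plus an era counter for extremely large year counts.
; While ticking, it adds delta time scaled by TimeMultiplier and rolls overflow up through minutes, hours and days, warning if one step reaches a minute.
; Day rollover uses month lengths with Gregorian leap-year rules.
; Setters control ticking and speed; getters return time and date combinations.
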(event EventTick
  (params (DeltaSeconds :type Float%20%28single-precision%29))
  (bind _timemultiplier (Variables|Default|GetTimeMultiplier))
  (bind _returnvalue (* DeltaSeconds _timemultiplier))
  (if (Variables|Default|GetIsTicking)
    (if (< _returnvalue 6e+01)
      (Variables|Default|SetSeconds (+ (Variables|Default|GetSeconds) _returnvalue))
      (if (>= (+ (Variables|Default|GetSeconds) _returnvalue) 6e+01)
        (Variables|Default|SetSeconds (- (Variables|Default|GetSeconds) 6e+01))
        (bind _result (Math|Float|IncrementFloat (Variables|Default|GetMinutes))
          (:%20%20
            (if (>= _result 6e+01)
              (Variables|Default|SetMinutes (- (Variables|Default|GetMinutes) 6e+01))
              (bind _result_2 (Math|Float|IncrementFloat (Variables|Default|GetHours))
                (:%20%20
                  (if (>= _result_2 24.0)
                    (Variables|Default|SetHours (- _result_2 24.0))
                    (CallFunction|IncrementDay))))))))
      (else
        (Development|PrintString "Single Delta is greater than one minute" true true "(R=1.000000,G=0.984000,B=0.000000,A=1.000000)")))))

(fn ConstructionScript)

(fn SetIsTicking
  (params (NewIsTicking :type Boolean))
  (Variables|Default|SetIsTicking NewIsTicking))

(fn IncrementDay
  (bind _numberofdays (CallFunction|GetNumberOfDaysinMonth (Variables|Default|GetYears) (Variables|Default|GetMonths)))
  (bind _result (Math|Float|IncrementFloat (Variables|Default|GetDays))
    (:%20%20
      (if (> _result _numberofdays)
        (Variables|Default|SetDays 1.0)
        (if (< (Variables|Default|GetMonths) 12.0)
          (Math|Float|IncrementFloat (Variables|Default|GetMonths)
            (:%20%20
              (Development|PrintString "New Month")))
          (else
            (Variables|Default|SetMonths 1.0)
            (bind _result_2 (Math|Float|IncrementFloat (Variables|Default|GetYears))
              (:%20%20
                (if (> _result_2 1e+12)
                  (Development|PrintString "Over 1000 billion years, new era")
                  (Math|Float|IncrementFloat (Variables|Default|GetEra)
                    (:%20%20
                      (Variables|Default|SetYears 0.0)))
                  (else
                    (Development|PrintString "New Year")))))))))))

(fn GetNumberOfDaysinMonth
  (params (Year :type Float%20%28double-precision%29) (Month :type Float%20%28double-precision%29))
  (if (== Month 2.0)
    (if (or (== (Math|Float|%(Float) Year 4e+02) 0.0) (and (== (Math|Float|%(Float) Year 4.0) 0.0) (!= (Math|Float|%(Float) Year 1e+02) 0.0)))
      (return 29.0)
      (else
        (return 28.0)))
    (elif (Math|Boolean|ORBoolean (== Month 1.0) (== Month 3.0) (== Month 5.0) (== Month 7.0) (== Month 8.0) (== Month 1e+01) (== Month 12.0))
      (return 31.0)
      (else
        (return 3e+01)))))

(fn GetDate
  (return (Variables|Default|GetYears) (Variables|Default|GetMonths) (Variables|Default|GetDays)))

(fn GetTime
  (return (Variables|Default|GetHours) (Variables|Default|GetMinutes) (Variables|Default|GetSeconds)))

(fn GetDatewithEra
  (return (Variables|Default|GetYears) (Variables|Default|GetMonths) (Variables|Default|GetDays) (Variables|Default|GetEra)))

(fn GetDateTime
  (return (Variables|Default|GetYears) (Variables|Default|GetMonths) (Variables|Default|GetDays) (Variables|Default|GetHours) (Variables|Default|GetMinutes) (Variables|Default|GetSeconds)))

(fn GetDateTimewithEra
  (return (Variables|Default|GetYears) (Variables|Default|GetMonths) (Variables|Default|GetDays) (Variables|Default|GetHours) (Variables|Default|GetMinutes) (Variables|Default|GetSeconds) (Variables|Default|GetEra)))

(fn SetTimeMultiplier
  (params (NewTimeMultiplier :type Float%20%28double-precision%29))
  (Variables|Default|SetTimeMultiplier NewTimeMultiplier))