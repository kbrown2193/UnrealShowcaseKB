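; BP_TimeMultiplierLever is a lever actor for stepping the game's time multiplier through a TimeSteps array.
; Increase and decrease events check TimeStepIndex bounds, then pass the selected step to GameTimeManager.SetTimeMultiplier.
; The decrease event also increments the index, and the increase check allows it to reach one past the last element.
; Lever rotation timeline and SetRelativeRotation nodes exist but are unconnected, so the lever does not animate.
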(event Custom|IncreaseTimeMultiplierStep
  (if (< (Variables|Default|GetTimeStepIndex) (Utilities|Array|Length (Variables|Default|GetTimeSteps)))
    (Math|Integer|IncrementInt (Variables|Default|GetTimeStepIndex)
      (:%20%20
        (Default|SetTimeMultiplier (Variables|Default|GetGameTimeManager) (Utilities|Array|Get(acopy) (Variables|Default|GetTimeSteps) (Variables|Default|GetTimeStepIndex)))))))

(event Custom|DecreaseTimeMultiplerStep
  (if (> (Variables|Default|GetTimeStepIndex) 0)
    (Math|Integer|IncrementInt (Variables|Default|GetTimeStepIndex)
      (:%20%20
        (Default|SetTimeMultiplier (Variables|Default|GetGameTimeManager) (Utilities|Array|Get(acopy) (Variables|Default|GetTimeSteps) (Variables|Default|GetTimeStepIndex)))))))

(event EventBeginPlay)

(event Collision|EventActorBeginOverlap
  (params (OtherActor :type Actor%20Object%20Reference)))

(event EventTick
  (params (DeltaSeconds :type Float%20%28single-precision%29)))

(fn ConstructionScript)