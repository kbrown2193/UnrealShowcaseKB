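; BP_WorldLightingManager rotates the sun's directional light to match the in-game time of day.
; While IsTicking is set, Tick reads the TimeManager's date-time and converts hours, minutes and seconds into pitch, scaled by a direction multiplier and shifted by a morning offset.
; Yaw stays at the configured level sun rotation.
; SwapDirectionalLightToSun is an empty stub, and a call zeroing light intensity is left unconnected.
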(event EventTick
  (params (DeltaSeconds :type Float%20%28single-precision%29))
  (bind _directionmultiplier (Variables|Default|GetDirectionMultiplier))
  (if (Variables|Default|GetIsTicking)
    (bind (_year _month _day _hours _minutes _seconds) (Default|GetDateTime (Variables|Default|GetTimeManager)))
    (Transformation|SetActorRotation (Variables|Default|GetSunDirectionalLight) (Math|Rotator|MakeRotator 0.0 (+ (* _hours 15.0 _directionmultiplier) (* _minutes 0.25 _directionmultiplier) (* _seconds 0.004167 _directionmultiplier) (Variables|Default|GetMorningOffset)) (Variables|Default|GetLevelSunLightZRotation)))))

(fn ConstructionScript)

(fn SwapDirectionalLighttoSun)