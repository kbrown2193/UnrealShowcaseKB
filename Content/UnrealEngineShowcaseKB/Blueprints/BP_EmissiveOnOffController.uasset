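; BP_EmissiveOnOffController switches a set of actors with emissive lights on, off or toggled as a group through BPI_EmissiveControl.
; On BeginPlay it casts each EmissiveOnOffActors entry to the interface, caches it and applies IsOn to the cached list after each success, printing an error for non-implementers.
; Custom events broadcast TurnOn, TurnOff, SetIsOn or ToggleOnOff to that cache.
; A delayed toggle test loop is left unconnected.
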(event Custom|TurnAllLightsOn
  (for _array_element (Variables|Default|GetEmissiveOnOffBPIs)
    (Default|Turnon _array_element)))

(event Custom|TurnAllLightsOff
  (for _array_element (Variables|Default|GetEmissiveOnOffBPIs)
    (Default|TurnOff _array_element)))

(event Custom|TurnAllLightsToIsOn
  (for _array_element (Variables|Default|GetEmissiveOnOffBPIs)
    (Default|SetIson _array_element (Variables|Default|GetIsOn))))

(event Custom|ToggleAllLights
  (for _array_element (Variables|Default|GetEmissiveOnOffBPIs)
    (Default|ToggleonOff _array_element)))

(event EventBeginPlay
  (for (_array_element _array_index) (Variables|Default|GetEmissiveOnOffActors)
    (bind _asbpi_emissive_control (Utilities|Casting|CastToBPI_EmissiveControl _array_element)
      (:then
        (Utilities|Array|SetArrayElem (Variables|Default|GetEmissiveOnOffBPIs) _array_index _asbpi_emissive_control true)
        (CallFunction|TurnAllLightstoIson))
      (:CastFailed
        (Development|PrintString "ERROR: Actir Not of Type BPI_EmissiveControl")))))

(fn ConstructionScript)