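; Test Blueprint for an emissive object that switches between on and off glow intensities, with adjustable color.
; Events set color, both intensities and the IsOn state, then refresh the affected value on EmissiveObject.
; Values reach the material through Custom Primitive Data, with color as a vector and intensity as a separate float.
; BeginPlay applies the initial state, and a debug key toggles it while printing IsOn before and after.
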(event EventBeginPlay
  (CallFunction|RefreshEmissiveColor)
  (CallFunction|RefreshEmissiveIntensity))

(event EventSetIson
  (params (NewIsOn :type Boolean))
  (Variables|Default|SetIsOn NewIsOn)
  (CallFunction|RefreshEmissiveIntensity))

(event EventSetEmissionColor
  (params (NewEmissiveColor :type Linear%20Color%20Structure))
  (Variables|Default|SetEmissiveColor NewEmissiveColor)
  (CallFunction|RefreshEmissiveColor))

(event EventSetonEmissionIntensity
  (params (NewOnEmissionIntensity :type Float%20%28double-precision%29))
  (Variables|Default|SetEmissiveOnIntensity NewOnEmissionIntensity)
  (CallFunction|RefreshEmissiveIntensity))

(event EventSetOffEmissionIntensity
  (params (NewOffEmissionIntensity :type Float%20%28double-precision%29))
  (Variables|Default|SetEmissiveOffIntensity NewOffEmissionIntensity)
  (CallFunction|RefreshEmissiveIntensity))

(event EventToggleonOff
  (if (Variables|Default|GetIsOn)
    (CallFunction|TurnOff)
    (else
      (CallFunction|Turnon))))

(event EventTurnOff
  (Variables|Default|SetIsOn false)
  (CallFunction|RefreshEmissiveIntensity))

(event EventTurnon
  (Variables|Default|SetIsOn true)
  (CallFunction|RefreshEmissiveIntensity))

(event Input|KeyboardEvents|DebugKey5
  (params (Key :type Key%20Structure :default "None") (ActionValue :type Input%20Action%20Value%20Structure))
  (bind _ison (Variables|Default|GetIsOn))
  (bind _returnvalue (Utilities|String|ToString(Boolean) _ison))
  (:Pressed
    (Development|PrintString (Utilities|String|Append "On start IsOn = " _returnvalue))
    (CallFunction|ToggleonOff)
    (Development|PrintString (Utilities|String|Append "On End IsOn = " _returnvalue))))

(fn ConstructionScript)

(fn RefreshEmissiveColor
  (bind _emissivecolor (Variables|Default|GetEmissiveColor))
  (Rendering|Material|SetCustomPrimitiveDataVector4 (Variables|Default|GetEmissiveObject) 0 (Math|Vector4|MakeVector4 (.r _emissivecolor) (.g _emissivecolor) (.b _emissivecolor) (.a _emissivecolor))))

(fn RefreshEmissiveIntensity
  (bind _emissiveobject (Variables|Default|GetEmissiveObject))
  (if (Variables|Default|GetIsOn)
    (Rendering|Material|SetCustomPrimitiveDataFloat _emissiveobject 4 (Variables|Default|GetEmissiveOnIntensity))
    (else
      (Rendering|Material|SetCustomPrimitiveDataFloat _emissiveobject 4 (Variables|Default|GetEmissiveOffIntensity)))))